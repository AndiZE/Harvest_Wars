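; Tooltips_BP is an interactable actor that shows an item information tooltip when the player presses E nearby.
; A Box overlap with a Character enables input on the actor for player 0, and ending the overlap disables it.
; Pressing E copies ContentToShow into the Tooltips_Widget of its widget component, then shows that widget for two seconds before hiding it.
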(event `Key|E`
  (params (Key :type "Key Structure"))
  (bind _widget (`self.Widget`))
  ;[1 1 1] Press E to get Item information for 2 seconds
  (:`Pressed`
    (bind _output_get (set `self.PromotedWidget` (`WidgetComponent.GetUserWidgetObject` (`self.Widget`))))
    (bind _astooltips_widget (cast `/Game/UserInterface/GUI/Tooltips/Tooltips_Widget` _output_get))
    (set `/Game/UserInterface/GUI/Tooltips/Tooltips_Widget.Content` (`self.ContentToShow`) _astooltips_widget)
    (`SceneComponent.SetVisibility` _widget true false)
    (`KismetSystemLibrary.Delay` 2.0)
    (`SceneComponent.SetVisibility` _widget false false)))

(event `self.Box.OnComponentBeginOverlap`
  (params (OverlappedComponent :type "PrimitiveComponent Object Reference") (OtherActor :type "Actor Object Reference") (OtherComp :type "PrimitiveComponent Object Reference") (OtherBodyIndex :type Integer) (bFromSweep :type Boolean) (SweepResult :type "HitResult Structure (by ref)"))
  (cast `Character` OtherActor)
  (`self.EnableInput` (`GameplayStatics.GetPlayerController` 0)))

(event `self.Box.OnComponentEndOverlap`
  (params (OverlappedComponent :type "PrimitiveComponent Object Reference") (OtherActor :type "Actor Object Reference") (OtherComp :type "PrimitiveComponent Object Reference") (OtherBodyIndex :type Integer))
  (cast `Character` OtherActor)
  (`self.DisableInput` (`GameplayStatics.GetPlayerController` 0)))

(fn `UserConstructionScript`)