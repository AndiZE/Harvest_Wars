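; Waypoint manager Blueprint that picks a random next destination for AI from a supplied set of waypoint actors.
; GetNextWaypoint returns a random waypoint's location, rerolling while it matches the current waypoint position within a small tolerance.
; The retry loop has no exit guard, so it never ends if every waypoint shares the current location, as with a single-entry array.
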(fn `GetNextWaypoint`
  (params (Waypoints :type "Array of /Game/Blueprints/AI/BP_Waypoint Object Reference") (CurrentWaypoint :type "Vector Structure"))
  (returns (NextWaypoint :type "Vector Structure"))
  (locals (Variable :type "Vector Structure"))
  (bind _waypoints (`local.Waypoints`))
  (bind _returnvalue (`self.K2_GetActorLocation` (`|GetArrayItem` _waypoints (`KismetMathLibrary.RandomIntegerInRange` 0 (`KismetArrayLibrary.Array_LastIndex` _waypoints)))))
  (bind _output_get (set `local.Variable` _returnvalue))
  (while (== _output_get CurrentWaypoint :`ErrorTolerance` 0.1)
    (set `local.Variable` _returnvalue))
  (return (`local.Variable`)))

(fn `UserConstructionScript`)