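; AI-driven Corn of Duty actor that walks to a target and plays footstep sounds as it moves.
; The MoveToTarget event issues a simple move-to-actor order toward TargetPosition.
; Every tick, PlayFootSound checks that velocity exceeds a small threshold and FootAudio is idle, then plays a random clip from StepSounds, so steps follow one another without overlapping.
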(event `MoveToTarget`
  (`AIBlueprintHelperLibrary.SimpleMoveToActor` null (`self.TargetPosition`)))

(event `self.ReceiveTick`
  (params (DeltaSeconds :type "Float (single-precision)"))
  (`self.PlayFootSound`))

(fn `PlayFootSound`
  (bind _stepsounds (`self.StepSounds`))
  (bind _footaudio (`self.FootAudio`))
  ;[1 1 1] FootSound
  (if (and (> (`KismetMathLibrary.VSize` (`self.GetVelocity`)) 0.3) (not (`AudioComponent.IsPlaying` _footaudio)))
    (`AudioComponent.SetSound` _footaudio (`|GetArrayItem` _stepsounds (`KismetMathLibrary.RandomIntegerInRange` 0 (`KismetArrayLibrary.Array_LastIndex` _stepsounds))))
    (`AudioComponent.Play` _footaudio 0.0)))

(fn `UserConstructionScript`)