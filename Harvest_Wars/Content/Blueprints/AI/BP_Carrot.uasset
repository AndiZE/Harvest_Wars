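; BP_Carrot is an AI-driven 2D carrot character that plays an animated spawn sequence before going idle.
; Spawn reveals the Paper2D sprite, plays the spawn flipbook once and plays a random spawn sound through the idle audio component.
; When the flipbook finishes, OnFinishedSpawn switches to the looping idle flipbook and sets the SpawnFinished blackboard key, signalling the AI that spawning is done.
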(event `self.ReceiveBeginPlay`
  (`parent.ReceiveBeginPlay`))

(fn `OnFinishedSpawn`
  (bind _sprite (`self.Sprite`))
  (bind _sprite_2 (`self.Sprite`))
  (clear `PaperFlipbookComponent.OnFinishedPlaying` _sprite)
  (`PaperFlipbookComponent.SetLooping` _sprite true)
  (`BlackboardComponent.SetValueAsBool` (`AIBlueprintHelperLibrary.GetBlackboard` self) "SpawnFinished" true)
  (`PaperFlipbookComponent.SetFlipbook` _sprite_2 "/Game/Assets/Enemy/Carrot/Idle/CarRot_Idle.CarRot_Idle")
  (`PaperFlipbookComponent.Play` _sprite_2))

(fn `Spawn`
  (bind _sprite (`self.Sprite`))
  (bind _spawnsound (`self.SpawnSound`))
  (bind _idleaudio (`self.IdleAudio`))
  (`SceneComponent.SetVisibility` (`self.Sprite`) true false)
  (`PaperFlipbookComponent.SetLooping` _sprite false)
  (`PaperFlipbookComponent.SetFlipbook` (`self.Sprite`) (`self.SpawnAnimation`))
  (add `PaperFlipbookComponent.OnFinishedPlaying` _sprite (`|CreateDelegate` :!event `OnFinishedSpawn`))
  (`AudioComponent.SetSound` _idleaudio (`|GetArrayItem` _spawnsound (`KismetMathLibrary.RandomIntegerInRange` 0 (`KismetArrayLibrary.Array_Length` _spawnsound))))
  (`AudioComponent.Play` _idleaudio 0.0))

(fn `UserConstructionScript`
  (`parent.UserConstructionScript`))