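; AI director for two-player combat that coordinates enemies so each player has one designated attacker at a time.
; Registers added enemies and sets their blackboard waypoints to random reachable points around players.
; A looping timer picks random non-attacking enemies for free living-player slots, flags their blackboards and orders attacks.
; Death handlers update these slots, stop the timer without players, and unlock the BP_LevelSetup camera once enemies are gone.
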(event `SendEnemy`
  (if (> (`KismetArrayLibrary.Array_Length` (`self.Enemies`)) 0)
    (`self.SendEnemyAttacking`)))

(event `self.ReceiveBeginPlay`
  (add `self.EnemyAdded` (`|CreateDelegate` :!event `OnEnemyAdded`)))

(event `On Player Added`
  (params (Players :type "Array of /Game/Blueprints/Character/BP_BasePlayerCharacter Object Reference"))
  ;[1 1 1] On Player Added
  (bind _output_get (set `self.Players` Players))
  (for _array_element _output_get
    (add `/Game/Blueprints/Character/HealthComponent.OnDie` (`/Game/Blueprints/Character/BP_BasePawn.HealthComponent` _array_element) (delegate `On Player Die`))
    (if (== (`/Game/Blueprints/Character/BP_BasePlayerCharacter.PlayerControllerID` _array_element) 0)
      (set `self.p1Alive` true)
      (else
        (set `self.p2Alive` true))))
  (bind _returnvalue (`KismetSystemLibrary.K2_SetTimerDelegate` (delegate `SendEnemy`) (`self.CheckInterval`) true))
  (set `self.AttackCheckTimer` _returnvalue))

(event `On Player Die`
  (bind _players (`self.Players`))
  ;[1 1 1] On Player Die
  (for _array_element _players
    (if (not (`/Game/Blueprints/Character/HealthComponent.IsAlive` (`/Game/Blueprints/Character/BP_BasePawn.HealthComponent` _array_element)))
      (`KismetArrayLibrary.Array_RemoveItem` (`self.Players`) _array_element)
      (if (== (`/Game/Blueprints/Character/BP_BasePlayerCharacter.PlayerControllerID` _array_element) 0)
        (set `self.p1Alive` false)
        (else
          (set `self.p2Alive` false)))))
  (if (== (`KismetArrayLibrary.Array_Length` _players) 0)
    (`KismetSystemLibrary.K2_ClearAndInvalidateTimerHandle` (`self.AttackCheckTimer`))))

(fn `GetRandomEnemy`
  (returns (Enemy :type "/Game/Blueprints/AI/BP_BaseAIPawn Object Reference"))
  (locals (TempAiPawn :type "/Game/Blueprints/AI/BP_BaseAIPawn Object Reference") (Overflowcounter :type Integer))
  (bind _enemies (`self.Enemies`))
  (bind _output (`|GetArrayItem` _enemies (`KismetMathLibrary.RandomIntegerInRange` 0 (`KismetArrayLibrary.Array_LastIndex` _enemies))))
  (bind _output_get (set `local.TempAiPawn` _output))
  (while (`BlackboardComponent.GetValueAsBool` (`AIBlueprintHelperLibrary.GetBlackboard` _output_get) (`self.BBKey_IsAttacking`))
    (set `local.TempAiPawn` _output)
    (bind _result (`/Engine/EditorBlueprintResources/StandardMacros.IncrementInt` (`local.Overflowcounter`))
      (:`  `
        (if (> _result 20)
          (return null)))))
  (return (`local.TempAiPawn`)))

(fn `GetRandomPlayer`
  (returns (Player :type "/Game/Blueprints/Character/BP_BasePlayerCharacter Object Reference"))
  (bind _players (`self.Players`))
  (return (`|GetArrayItem` _players (`KismetMathLibrary.RandomIntegerInRange` 0 (`KismetArrayLibrary.Array_LastIndex` _players)))))

(fn `GetRandomPointAroundPlayer`
  (params (Player :type "/Game/Blueprints/Character/BP_BasePlayerCharacter Object Reference") (MinDistance :type "Float (double-precision)") (MaxDistance :type "Float (double-precision)"))
  (returns (Location :type "Vector Structure") (Success :type Boolean))
  (bind (_randomlocation _returnvalue) (`NavigationSystemV1.K2_GetRandomReachablePointInRadius` (`self.K2_GetActorLocation` Player) MaxDistance null null))
  (`/Engine/EditorBlueprintResources/StandardMacros.IsValid` Player
    (:`Is Valid`
      (return _randomlocation _returnvalue))))

(fn `OnEnemyAdded`
  (params (Enemy :type "/Game/Blueprints/AI/BP_BaseAIPawn Object Reference"))
  (locals (Location :type "Vector Structure") (success :type Boolean))
  (bind _enemy (`local.Enemy`))
  (`/Engine/EditorBlueprintResources/StandardMacros.IsValid` Enemy
    (:`Is Valid`
      (set `/Game/Blueprints/AI/BP_BaseAIPawn.AiHandler` self Enemy)
      (`KismetArrayLibrary.Array_Add` (`self.Enemies`) _enemy)
      (`self.SetRandomWaypoint` _enemy 400.0 800.0))))

(fn `OnEnemyDied`
  (params (Enemy :type "/Game/Blueprints/AI/BP_BaseAIPawn Object Reference"))
  (if (`KismetArrayLibrary.Array_Contains` (`self.Enemies`) Enemy)
    (`KismetArrayLibrary.Array_RemoveItem` (`self.Enemies`) Enemy)
    (if (== (`self.p1Enemy`) (`local.Enemy`))
      (set `self.p1Enemy` null)
      (set `self.p1Attacking` false)
      (elif (not (== (`self.p2Enemy`) (`local.Enemy`)))
        (set `self.p2Enemy` null)
        (set `self.p2Attacking` false)))
    (if (== (`KismetArrayLibrary.Array_Length` (`self.Enemies`)) 0)
      (bind _outactors (`GameplayStatics.GetAllActorsOfClass` "/Game/Blueprints/Level/BP_LevelSetup.BP_LevelSetup_C"))
      (`/Game/Blueprints/Level/BP_LevelSetup.UnlockCamera` (`|GetArrayItem` _outactors)))))

(fn `SendEnemyAttacking`
  (locals (TempAI :type "/Game/Blueprints/AI/BP_BaseAIPawn Object Reference") (TempPlayer :type "/Game/Blueprints/Character/BP_BasePlayerCharacter Object Reference") (counter :type Integer))
  (bind _tempai (`local.TempAI`))
  (bind _p2enemy (`self.p2Enemy`))
  (bind _p2enemy_2 (`self.p2Enemy`))
  (bind _tempai_2 (`local.TempAI`))
  (if (and (not (`self.p1Attacking`)) (`self.p1Alive`))
    ;[1 1 1] P1
    (set `local.TempAI` (`self.GetRandomEnemy`))
    (while (and (`KismetMathLibrary.BooleanNOR` (`KismetSystemLibrary.IsValid` _p2enemy_2) (!= _p2enemy_2 (`local.TempAI`))) (< (`local.counter`) 11))
      (set `local.TempAI` (`self.GetRandomEnemy`))
      (`/Engine/EditorBlueprintResources/StandardMacros.IncrementInt` (`local.counter`)))
    (`/Engine/EditorBlueprintResources/StandardMacros.IsValid` _tempai
      (:`Is Valid`
        (set `self.p1Enemy` _tempai)
        (set `self.p1Attacking` true)
        (`BlackboardComponent.SetValueAsBool` (`AIBlueprintHelperLibrary.GetBlackboard` (`self.p1Enemy`)) (`self.BBKey_IsAttacking`) true)
        (bind _asbp_base_player_character (cast `/Game/Blueprints/Character/BP_BasePlayerCharacter` (`Controller.K2_GetPawn` (`GameplayStatics.GetPlayerController` 0))))
        (`/Game/Blueprints/AI/BP_BaseAIPawn.AttackPlayer` (`self.p1Enemy`) _asbp_base_player_character)))
    (elif (and (not (`self.p2Attacking`)) (`self.p2Alive`))
      ;[1 1 1] P2
      (set `local.TempAI` (`self.GetRandomEnemy`))
      (while (and (`KismetMathLibrary.BooleanNOR` (`KismetSystemLibrary.IsValid` _p2enemy) (!= _p2enemy (`local.TempAI`))) (< (`local.counter`) 11))
        (set `local.TempAI` (`self.GetRandomEnemy`))
        (`/Engine/EditorBlueprintResources/StandardMacros.IncrementInt` (`local.counter`)))
      (`/Engine/EditorBlueprintResources/StandardMacros.IsValid` _tempai_2
        (:`Is Valid`
          (set `self.p2Enemy` _tempai_2)
          (set `self.p2Attacking` true)
          (`BlackboardComponent.SetValueAsBool` (`AIBlueprintHelperLibrary.GetBlackboard` (`self.p2Enemy`)) (`self.BBKey_IsAttacking`) true)
          (bind _asbp_base_player_character_2 (cast `/Game/Blueprints/Character/BP_BasePlayerCharacter` (`Controller.K2_GetPawn` (`GameplayStatics.GetPlayerController` 1))))
          (`/Game/Blueprints/AI/BP_BaseAIPawn.AttackPlayer` (`self.p2Enemy`) _asbp_base_player_character_2))))))

(fn `SetRandomWaypoint`
  (params (Enemy :type "/Game/Blueprints/AI/BP_BaseAIPawn Object Reference") (Min :type "Float (double-precision)") (Max :type "Float (double-precision)"))
  (locals (Success :type Boolean) (Location :type "Vector Structure"))
  (bind (_location _success) (`self.GetRandomPointAroundPlayer` (`self.GetRandomPlayer`) Min Max))
  (bind _returnvalue (not _success))
  (if (> (`KismetArrayLibrary.Array_Length` (`self.Players`)) 0)
    (set `local.Location` _location)
    (bind _output_get (set `local.success` _returnvalue))
    (while _output_get
      (set `local.Location` _location)
      (set `local.success` _returnvalue))
    (`BlackboardComponent.SetValueAsVector` (`AIBlueprintHelperLibrary.GetBlackboard` (`local.Enemy`)) (`self.BBKey_Waypoint`) (`local.Location`))))

(fn `UserConstructionScript`)