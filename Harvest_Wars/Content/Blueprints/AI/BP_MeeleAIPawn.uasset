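; Melee enemy AI pawn that damages player characters with box-overlap attacks in a sprite-based setup.
; On BeginPlay it flags SpawnFinished in the blackboard when it has no spawn animation.
; AttackEnemy sweeps the weapon sprite's bounds if armed, otherwise a box offset toward its facing side.
; Hits are filtered by Y-axis distance, with different threshold checks per branch, then DamageComponent's calculated damage goes to the player's HealthComponent.
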(event `self.ReceiveBeginPlay`
  (`parent.ReceiveBeginPlay`)
  (if (not (`self.HasSpawnAnimation`))
    (`BlackboardComponent.SetValueAsBool` (`AIBlueprintHelperLibrary.GetBlackboard` null) "SpawnFinished" true)))

(event `self.AttackEnemy`
  (bind (_returnvalue_x _returnvalue_y) (`KismetMathLibrary.BreakVector` (`self.K2_GetActorLocation`)))
  (bind (_returnvalue_x_2 _returnvalue_y_2) (`KismetMathLibrary.BreakVector` (`self.K2_GetActorLocation`)))
  (bind _attackspriteextent_x (`KismetMathLibrary.BreakVector` (`self.AttackSpriteExtent`)))
  (bind _attackspriteextent_x_2 (`KismetMathLibrary.BreakVector` (`self.AttackSpriteExtent`)))
  (bind (_origin _boxextent) (`KismetSystemLibrary.GetComponentBounds` (`self.WeaponSprite`)))
  (if (`self.HasWeapon`)
    (bind (_outactors _returnvalue) (`KismetSystemLibrary.BoxOverlapActors` _origin _boxextent (`|MakeArray` "ObjectTypeQuery3" :!type "EObjectTypeQuery Enum") "/Game/Blueprints/Character/BP_BasePlayerCharacter.BP_BasePlayerCharacter_C" (`|MakeArray` self :!type "Actor Object Reference")))
    (if _returnvalue
      (for _array_element _outactors
        (bind _asbp_base_player_character (cast `/Game/Blueprints/Character/BP_BasePlayerCharacter` _array_element))
        (bind (_returnvalue_x_3 _returnvalue_y_3) (`KismetMathLibrary.BreakVector` (`self.K2_GetActorLocation` _asbp_base_player_character)))
        (if (<= (`KismetMathLibrary.Abs` (- _returnvalue_y _returnvalue_y_3)) (`self.HitTresholdMin`))
          (`/Game/Blueprints/Character/HealthComponent.DamageRecieve` (`/Game/Blueprints/Character/BP_BasePawn.HealthComponent` _asbp_base_player_character) (`/Game/Blueprints/Character/DamageComponent.CalculateDamage` (`self.DamageComponent`))))))
    (else
      (bind (_outactors_2 _returnvalue_2) (`KismetSystemLibrary.BoxOverlapActors` (select `bool` (`self.IsRight`) :`false` (+ (`self.K2_GetActorLocation`) (`KismetMathLibrary.MakeVector` (* _attackspriteextent_x -1.0))) :`true` (+ (`self.K2_GetActorLocation`) (`KismetMathLibrary.MakeVector` _attackspriteextent_x_2))) (`self.AttackSpriteExtent`) (`|MakeArray` "ObjectTypeQuery3" :!type "EObjectTypeQuery Enum") "/Game/Blueprints/Character/BP_BasePlayerCharacter.BP_BasePlayerCharacter_C" (`|MakeArray` self :!type "Actor Object Reference")))
      (if _returnvalue_2
        (for _array_element_2 _outactors_2
          (bind _asbp_base_player_character_2 (cast `/Game/Blueprints/Character/BP_BasePlayerCharacter` _array_element_2))
          (bind (_returnvalue_x_4 _returnvalue_y_4) (`KismetMathLibrary.BreakVector` (`self.K2_GetActorLocation` _asbp_base_player_character_2)))
          (bind _returnvalue_3 (- _returnvalue_y_2 _returnvalue_y_4))
          (if (and (> _returnvalue_3 (`self.HitTresholdMin`)) (< _returnvalue_3 (`self.HitTresholdMax`)))
            (`/Game/Blueprints/Character/HealthComponent.DamageRecieve` (`/Game/Blueprints/Character/BP_BasePawn.HealthComponent` _asbp_base_player_character_2) (`/Game/Blueprints/Character/DamageComponent.CalculateDamage` (`self.DamageComponent`)))))))))

(fn `UserConstructionScript`
  (`parent.UserConstructionScript`))