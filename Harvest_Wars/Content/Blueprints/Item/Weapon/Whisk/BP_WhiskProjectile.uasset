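; Whisk weapon projectile that adds a spinning motion on top of its parent class's behavior.
; On BeginPlay it picks a random spin speed between MinRot and MaxRot and a random starting yaw, so each projectile looks different.
; Tick advances the yaw by that speed scaled by delta time, keeping pitch and roll unchanged.
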(event `self.ReceiveBeginPlay`
  (bind (_returnvalue_roll _returnvalue_pitch) (`KismetMathLibrary.BreakRotator` (`self.K2_GetActorRotation`)))
  (`parent.ReceiveBeginPlay`)
  (set `self.RotationSpeed` (`KismetMathLibrary.RandomFloatInRange` (`self.MinRot`) (`self.MaxRot`)))
  (`self.K2_SetActorRotation` (`KismetMathLibrary.MakeRotator` _returnvalue_roll _returnvalue_pitch (`KismetMathLibrary.RandomFloatInRange` 0.0 359.0))))

(event `self.ReceiveTick`
  (params (DeltaSeconds :type "Float (single-precision)"))
  (bind (_returnvalue_roll _returnvalue_pitch _returnvalue_yaw) (`KismetMathLibrary.BreakRotator` (`self.K2_GetActorRotation`)))
  (`self.K2_SetActorRotation` (`KismetMathLibrary.MakeRotator` _returnvalue_roll _returnvalue_pitch (+ (* DeltaSeconds (`self.RotationSpeed`)) _returnvalue_yaw))))

(fn `UserConstructionScript`
  (`parent.UserConstructionScript`))