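; Base projectile actor for weapons that deals damage to pawns it hits.
; Init stores the damage and launches the render component with a velocity-change impulse along the given direction scaled by Speed.
; On component hit, it casts the other actor to BP_BasePawn, passes Damage to that pawn's HealthComponent and destroys itself; hits on other actors leave it alive.
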(event `self.RenderComponent.OnComponentHit`
  (params (HitComponent :type "PrimitiveComponent Object Reference") (OtherActor :type "Actor Object Reference") (OtherComp :type "PrimitiveComponent Object Reference") (NormalImpulse :type "Vector Structure") (Hit :type "HitResult Structure (by ref)"))
  (bind _asbp_base_pawn (cast `/Game/Blueprints/Character/BP_BasePawn` OtherActor))
  (`/Game/Blueprints/Character/HealthComponent.DamageRecieve` (`/Game/Blueprints/Character/BP_BasePawn.HealthComponent` _asbp_base_pawn) (`self.Damage`))
  (`self.K2_DestroyActor`))

(fn `Init`
  (params (Damage :type Integer) (Direction :type "Vector Structure"))
  (`PrimitiveComponent.AddImpulse` (`self.RenderComponent`) (* Direction (`self.Speed`)) "None" true)
  (set `self.Damage` (`local.Damage`)))

(fn `UserConstructionScript`)