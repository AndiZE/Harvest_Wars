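; BP_Consumable is a consumable item pickup that a player character collects by overlapping its sprite.
; When level-placed, it loads its item data from the consumable DataTable row, printing a warning if the handle points at another table.
; The construction script and BeginPlay both apply the item's sprite.
; Pawn-component overlaps with a player who has a free inventory slot call PickupItem, then destroy the actor.
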(event `self.ReceiveBeginPlay`
  (bind (_item_name _item_sprite) (break `/Game/Blueprints/Item/Consumable/Consumable` (`self.Item`)))
  (`parent.ReceiveBeginPlay`)
  (if (`self.LevelPlaced`)
    (`self.Validate Debug Item`))
  (`PaperSpriteComponent.SetSprite` (`self.RenderComponent`) _item_sprite))

(event `self.RenderComponent.OnComponentBeginOverlap`
  (params (OverlappedComponent :type "PrimitiveComponent Object Reference") (OtherActor :type "Actor Object Reference") (OtherComp :type "PrimitiveComponent Object Reference") (OtherBodyIndex :type Integer) (bFromSweep :type Boolean) (SweepResult :type "HitResult Structure (by ref)"))
  (bind _asbp_base_player_character (cast `/Game/Blueprints/Character/BP_BasePlayerCharacter` OtherActor))
  (if (and (`/Game/Blueprints/Character/BP_BasePlayerCharacter.HasFreeInventorySlot` _asbp_base_player_character) (`|EnumEquality` (`PrimitiveComponent.GetCollisionObjectType` OtherComp) "ECC_Pawn"))
    (`/Game/Blueprints/Character/BP_BasePlayerCharacter.PickupItem` _asbp_base_player_character self)
    (`self.K2_DestroyActor` self)))

(fn `UserConstructionScript`
  (bind (_item_name _item_sprite) (break `/Game/Blueprints/Item/Consumable/Consumable` (`self.Item`)))
  (`parent.UserConstructionScript`)
  (if (`self.LevelPlaced`)
    (`self.Validate Debug Item`)
    (`PaperSpriteComponent.SetSprite` (`self.RenderComponent`) _item_sprite)))

(fn `Validate Debug Item`
  (bind (_itemhandle_datatable _itemhandle_rowname) (break `DataTableRowHandle` (`self.ItemHandle`)))
  (if (!= _itemhandle_datatable "/Game/Blueprints/Item/Consumable/ConsumableTable.ConsumableTable")
    (`KismetSystemLibrary.PrintString` (`KismetStringLibrary.Concat_StrStr` (`KismetSystemLibrary.GetDisplayName` self) "is Invalid Table! Set to Consumables!") true true (struct :`R` 1.0 :`A` 1.0) 4.0)
    (else
      (bind _returnvalue (`|GetDataTableRow` "/Game/Blueprints/Item/Consumable/ConsumableTable.ConsumableTable" _itemhandle_rowname)
        (:`then`
          (set `self.Item` _returnvalue))))))