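; BP_CornSpawn is a level trigger that starts a one-time Corn of Duty encounter once all players are inside its area.
; Overlap events track player characters in a list, and spawning fires when the count matches the GameInstance's MaxPlayers.
; It locks the camera through BP_LevelSetup, spawns BP_CornOfDuty at the spawn point, and sends it toward Destination via AI move, also setting that as its target.
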(event `self.TriggerArea.OnComponentBeginOverlap`
  (params (OverlappedComponent :type "PrimitiveComponent Object Reference") (OtherActor :type "Actor Object Reference") (OtherComp :type "PrimitiveComponent Object Reference") (OtherBodyIndex :type Integer) (bFromSweep :type Boolean) (SweepResult :type "HitResult Structure (by ref)"))
  (bind _asbp_base_player_character (cast `/Game/Blueprints/Character/BP_BasePlayerCharacter` OtherActor))
  (`KismetArrayLibrary.Array_AddUnique` (`self.Players`) _asbp_base_player_character)
  (bind _asbp_game_instance (cast `/Game/Gamemode/BP_GameInstance` (`GameplayStatics.GetGameInstance`)))
  (if (and (== (`/Game/Gamemode/BP_GameInstance.MaxPlayers` _asbp_game_instance) (`KismetArrayLibrary.Array_Length` (`self.Players`))) (not (`self.SpawnActive`)))
    (set `self.SpawnActive` true)
    (`self.SpawnCorn`)))

(event `self.TriggerArea.OnComponentEndOverlap`
  (params (OverlappedComponent :type "PrimitiveComponent Object Reference") (OtherActor :type "Actor Object Reference") (OtherComp :type "PrimitiveComponent Object Reference") (OtherBodyIndex :type Integer))
  (bind _players (`self.Players`))
  (bind _asbp_base_player_character (cast `/Game/Blueprints/Character/BP_BasePlayerCharacter` OtherActor))
  (if (`KismetArrayLibrary.Array_Contains` _players _asbp_base_player_character)
    (`KismetArrayLibrary.Array_RemoveItem` _players _asbp_base_player_character)))

(event `SpawnCorn`
  (bind _destination (`self.Destination`))
  (bind _outactors (`GameplayStatics.GetAllActorsOfClass` "/Game/Blueprints/Level/BP_LevelSetup.BP_LevelSetup_C"))
  (`/Game/Blueprints/Level/BP_LevelSetup.LockCamera` (`|GetArrayItem` _outactors) (`SceneComponent.K2_GetComponentLocation` (`self.CameraLockPosition`)))
  (bind _returnvalue (`|SpawnActorFromClass` "/Game/Blueprints/AI/BP_CornOfDuty.BP_CornOfDuty_C" (`KismetMathLibrary.MakeTransform` (`SceneComponent.K2_GetComponentLocation` (`self.SpawnPoint`)) (struct :`Roll` -90.0) (1.5 1.5 1.5)) "Undefined" "OverrideRootScale" null null))
  (`AIBlueprintHelperLibrary.SimpleMoveToActor` (`AIBlueprintHelperLibrary.GetAIController` _returnvalue) _destination)
  (set `/Game/Blueprints/AI/BP_CornOfDuty.TargetPosition` _destination _returnvalue))

(fn `UserConstructionScript`)