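; Level setup actor that creates the HUD, spawns local players and serves as their shared orthographic camera.
; BeginPlay takes the player count from BP_GameInstance or debug settings, spawns possessed characters at random PlayerStarts and destroys uncontrolled ones.
; Tick follows a lone player at fixed zoom, or centers on the players' average position, zooming by the first two players' distance.
; Camera Y is clamped to borders matching the zoom.
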(event `CameraSetupSingleplayer`
  (bind (_cameradistance_x _cameradistance_y) (`KismetMathLibrary.BreakVector2D` (`self.CameraDistance`)))
  (bind (_zoominborder_x _zoominborder_y) (`KismetMathLibrary.BreakVector2D` (`self.ZoomInBorder`)))
  (bind (_zoomoutborder_x _zoomoutborder_y) (`KismetMathLibrary.BreakVector2D` (`self.ZoomOutBorder`)))
  ;[1 1 1] Singeplayer Camera Setup
  (`CameraComponent.SetOrthoWidth` (`self.PlayerCam`) (/ (+ _cameradistance_x _cameradistance_y) 2.0))
  (set `self.SinglePlayerzoomBorder` (`KismetMathLibrary.MakeVector2D` (/ (+ _zoominborder_x _zoomoutborder_x) 2.0) (/ (+ _zoominborder_y _zoomoutborder_y) 2.0))))

(event `self.ReceiveBeginPlay`
  (bind _debugplayer (`self.DebugPlayer`))
  ;[1 1 1] Init
  (bind _returnvalue (`|CreateWidget` "/Game/UI/HUD/HUD.HUD_C" (`GameplayStatics.GetPlayerController` 0)))
  (bind _output_get (set `self.PlayerHUD` _returnvalue))
  (`UserWidget.AddToViewport` _output_get 0)
  (if (`self.DebugStart`)
    (`/Game/UI/HUD/HUD.Init` (`self.PlayerHUD`) _debugplayer)
    (`self.SetupPlayers` _debugplayer)
    (if (== _debugplayer 1)
      (`self.CameraSetupSingleplayer`))
    (else
      (bind _asbp_game_instance (cast `/Game/Gamemode/BP_GameInstance` (`GameplayStatics.GetGameInstance`)))
      (bind _maxplayers (`/Game/Gamemode/BP_GameInstance.MaxPlayers` _asbp_game_instance))
      (`/Game/UI/HUD/HUD.Init` (`self.PlayerHUD`) _maxplayers)
      (`self.SetupPlayers` _maxplayers)
      (if (== _maxplayers 1)
        (`self.CameraSetupSingleplayer`)))))

(event `SetupPlayers`
  (params (NumberPlayers :type Integer))
  ;[1 1 1] Setup Player
  (if (> NumberPlayers 1)
    (for _index (range NumberPlayers)
      (bind _returnvalue (`GameplayStatics.CreatePlayer` _index))
      (`GameplayStatics.SetPlayerControllerID` _returnvalue _index)
      (`self.AddPlayer` _index))
    (else
      (`GameplayStatics.CreatePlayer` 0)
      (`GameplayStatics.SetPlayerControllerID` null)
      (`self.AddPlayer` 0)))
  (`PlayerController.SetViewTargetWithBlend` (`GameplayStatics.GetPlayerController` 0) self 0.0 "VTBlend_Linear" 0.0 false)
  ;[0 1 0] Remove Default Level Spawed Actor, TODO: Should Resolve is possible
  (bind _outactors (`GameplayStatics.GetAllActorsOfClass` "/Game/Blueprints/Character/BP_BasePlayerCharacter.BP_BasePlayerCharacter_C"))
  (for _array_element _outactors
    (if (not (`Pawn.IsPlayerControlled` _array_element))
      (`self.K2_DestroyActor` _array_element))))

(event `AddPlayer`
  (params (ID :type Integer))
  (bind _returnvalue (`GameplayStatics.GetPlayerController` ID))
  (bind (_cameradistance_x _cameradistance_y) (`KismetMathLibrary.BreakVector2D` (`self.CameraDistance`)))
  ;[1 1 1] Add Player to Level and Save for Camera Logic
  (`/Engine/EditorBlueprintResources/StandardMacros.IsValid` _returnvalue
    (:`Is Valid`
      (bind _outactors (`GameplayStatics.GetAllActorsOfClass` "/Script/Engine.PlayerStart"))
      (bind _returnvalue_2 (`|SpawnActorFromClass` "/Game/Blueprints/Character/BP_BasePlayerCharacter.BP_BasePlayerCharacter_C" (`self.GetTransform` (`|GetArrayItem` _outactors (`KismetMathLibrary.RandomIntegerInRange` 0 (- (`KismetArrayLibrary.Array_Length` _outactors) 1)))) "AdjustIfPossibleButAlwaysSpawn" "OverrideRootScale" null ID (`self.Scene`) _cameradistance_y (`self.PlayerHUD`) null))
      (`/Engine/EditorBlueprintResources/StandardMacros.IsValid` _returnvalue_2
        (:`Is Valid`
          (`Controller.Possess` _returnvalue _returnvalue_2)
          (`WidgetBlueprintLibrary.SetInputMode_GameOnly` _returnvalue)
          (`KismetArrayLibrary.Array_Add` (`self.Players`) _returnvalue_2)
          (`/Engine/EditorBlueprintResources/StandardMacros.IncrementInt` (`self.NumberPlayers`)
            (:`  `
              (`/Game/UI/HUD/HUD.BindToPlayer` (`self.PlayerHUD`) _returnvalue_2)
              (`/Game/Blueprints/Character/BP_BasePlayerCharacter.Init` _returnvalue_2))))))
    (:`Is Not Valid`
      (`KismetSystemLibrary.PrintString` (`KismetStringLibrary.Concat_StrStr` "Invalid Controller Recieved with Playerindex: " (`KismetStringLibrary.Conv_IntToString` ID)) true true (struct :`R` 1.0 :`A` 1.0) 10.0))))

(event `self.ReceiveTick`
  (params (DeltaSeconds :type "Float (single-precision)"))
  (bind (_returnvalue_x _returnvalue_y _returnvalue_z) (`KismetMathLibrary.BreakVector` (`self.K2_GetActorLocation`)))
  (bind (_cameradistance_x _cameradistance_y) (`KismetMathLibrary.BreakVector2D` (`self.CameraDistance`)))
  (bind (_zoominborder_x _zoominborder_y) (`KismetMathLibrary.BreakVector2D` (`self.ZoomInBorder`)))
  (bind (_zoomoutborder_x _zoomoutborder_y) (`KismetMathLibrary.BreakVector2D` (`self.ZoomOutBorder`)))
  (bind (_singleplayerzoomborder_x _singleplayerzoomborder_y) (`KismetMathLibrary.BreakVector2D` (`self.SinglePlayerzoomBorder`)))
  (bind _players (`self.Players`))
  (bind (_returnvalue_x_2 _returnvalue_y_2 _returnvalue_z_2) (`KismetMathLibrary.BreakVector` (`self.K2_GetActorLocation` (`|GetArrayItem` (`self.Players`)))))
  (bind _returnvalue (`KismetMathLibrary.FClamp` (/ (`KismetMathLibrary.Vector_Distance` (`self.K2_GetActorLocation` (`|GetArrayItem` _players)) (`self.K2_GetActorLocation` (`|GetArrayItem` _players 1))) (/ _cameradistance_y 2.0))))
  ;[1 1 1] Cam Logic
  (if (> (`self.NumberPlayers`) 1)
    ;;[1 0 0] Multiplayer
    (set `self.LocationBuffer` (0.0 0.0 0.0))
    (for _array_element (`self.Players`)
      (set `self.LocationBuffer` (+ (`self.LocationBuffer`) (`self.K2_GetActorLocation` _array_element))))
    (`self.K2_SetActorLocation` (/ (`self.LocationBuffer`) (`self.NumberPlayers`)))
    ;[1 1 1] Multiplayer Camera Dynamic Zoom with Clamping
    (`CameraComponent.SetOrthoWidth` (`self.PlayerCam`) (`KismetMathLibrary.Lerp` _cameradistance_x _cameradistance_y _returnvalue))
    (`self.K2_SetActorLocation` (`KismetMathLibrary.MakeVector` _returnvalue_x (`KismetMathLibrary.FClamp` _returnvalue_y (`KismetMathLibrary.Lerp` _zoominborder_x _zoomoutborder_x _returnvalue) (`KismetMathLibrary.Lerp` _zoominborder_y _zoomoutborder_y _returnvalue)) _returnvalue_z)) ; Clamping Camera Location
    (else
      ;;[1 0 0] Singleplayer
      (`self.K2_SetActorLocation` (`KismetMathLibrary.MakeVector` _returnvalue_x_2 (`KismetMathLibrary.FClamp` _returnvalue_y_2 _singleplayerzoomborder_x _singleplayerzoomborder_y) _returnvalue_z_2)))))

(fn `UserConstructionScript`)