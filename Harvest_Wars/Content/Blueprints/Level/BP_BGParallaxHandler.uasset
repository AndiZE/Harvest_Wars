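; Level actor that drives a layered parallax background of BP_ParallaxObject sprites along the X axis.
; On BeginPlay it gathers placed objects and spawns a copy of each one LayerWidth to either side, with a random sprite from that layer's pool.
; Every tick it shifts all render components by the X movement of the BP_LevelSetup actor, scaled by layer number and LayerMultiplier.
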(event `self.ReceiveBeginPlay`
  (bind _outactors (`GameplayStatics.GetAllActorsOfClass` "/Game/Blueprints/Level/BP_LevelSetup.BP_LevelSetup_C"))
  (bind _output_get (set `self.Fokus` (`|GetArrayItem` _outactors)))
  (bind _returnvalue_x (`KismetMathLibrary.BreakVector` (`self.K2_GetActorLocation` _output_get)))
  (set `self.LastPositionX` _returnvalue_x)
  (bind _outactors_2 (`GameplayStatics.GetAllActorsOfClass` "/Game/Blueprints/Level/BP_ParallaxObject.BP_ParallaxObject_C"))
  (for _array_element _outactors_2
    (`KismetArrayLibrary.Array_AddUnique` (`self.ParallaxObjects`) _array_element))
  (for _array_element_2 (`self.ParallaxObjects`)
    (`|ExecutionSequence`
      (:`then_0`
        (bind (_returnvalue_x_2 _returnvalue_y _returnvalue_z) (`KismetMathLibrary.BreakVector` (`self.K2_GetActorLocation` _array_element_2)))
        (bind _layer (`/Game/Blueprints/Level/BP_ParallaxObject.Layer` _array_element_2))
        (bind _layeroffset (`/Game/Blueprints/Level/BP_ParallaxObject.LayerOffset` _array_element_2))
        (bind _returnvalue (`|SpawnActorFromClass` "/Game/Blueprints/Level/BP_ParallaxObject.BP_ParallaxObject_C" (`KismetMathLibrary.Conv_VectorToTransform` (`KismetMathLibrary.MakeVector` (+ _returnvalue_x_2 (`self.LayerWidth`)) _returnvalue_y _returnvalue_z)) "Undefined" "OverrideRootScale" null _layer _layeroffset null))
        (`self.SetupObject` _returnvalue)
        (`KismetArrayLibrary.Array_Add` (`self.TempList`) _returnvalue))
      (:`then_1`
        (bind (_returnvalue_x_3 _returnvalue_y_2 _returnvalue_z_2) (`KismetMathLibrary.BreakVector` (`self.K2_GetActorLocation` _array_element_2)))
        (bind _returnvalue_2 (`|SpawnActorFromClass` "/Game/Blueprints/Level/BP_ParallaxObject.BP_ParallaxObject_C" (`KismetMathLibrary.Conv_VectorToTransform` (`KismetMathLibrary.MakeVector` (- _returnvalue_x_3 (`self.LayerWidth`)) _returnvalue_y_2 _returnvalue_z_2)) "Undefined" "OverrideRootScale" null _layer _layeroffset null))
        (`self.SetupObject` _returnvalue_2)
        (`KismetArrayLibrary.Array_Add` (`self.TempList`) _returnvalue_2))))
  (for _array_element_3 (`self.TempList`)
    (`KismetArrayLibrary.Array_Add` (`self.ParallaxObjects`) _array_element_3))
  (`KismetArrayLibrary.Array_Clear` (`self.TempList`)))

(event `self.ReceiveTick`
  (params (DeltaSeconds :type "Float (single-precision)"))
  (`self.UpdatePositions`))

(fn `GetRandomLayerSprite`
  (params (Layer :type Integer))
  (returns (Sprite :type "PaperSprite Object Reference"))
  (bind _layer3 (`self.Layer3`))
  (bind _layer1 (`self.Layer1`))
  (bind _layer2 (`self.Layer2`))
  (bind _layer4 (`self.Layer4`))
  (switch `int` Layer
    (:`-1`
      (`KismetSystemLibrary.PrintString` "Layer -1 Not Assigned")
      (return "/Game/Debug/Helper-Icons/DebugSprite.DebugSprite"))
    (:`0`
      (`KismetSystemLibrary.PrintString` "Layer 0 (Player) not Assigned")
      (return "/Game/Debug/Helper-Icons/DebugSprite.DebugSprite"))
    (:`1`
      (return (`|GetArrayItem` _layer1 (`KismetMathLibrary.RandomIntegerInRange` 0 (`KismetArrayLibrary.Array_LastIndex` _layer1)))))
    (:`2`
      (return (`|GetArrayItem` _layer2 (`KismetMathLibrary.RandomIntegerInRange` 0 (`KismetArrayLibrary.Array_LastIndex` _layer2)))))
    (:`3`
      (return (`|GetArrayItem` _layer3 (`KismetMathLibrary.RandomIntegerInRange` 0 (`KismetArrayLibrary.Array_LastIndex` _layer3)))))
    (:`4`
      (return (`|GetArrayItem` _layer4 (`KismetMathLibrary.RandomIntegerInRange` 0 (`KismetArrayLibrary.Array_LastIndex` _layer4)))))))

(fn `SetupObject`
  (params (Object :type "/Game/Blueprints/Level/BP_ParallaxObject Object Reference"))
  (bind _rendercomponent (`PaperSpriteActor.RenderComponent` Object))
  (bind _sprite (`self.GetRandomLayerSprite` (`/Game/Blueprints/Level/BP_ParallaxObject.Layer` Object)))
  (`PaperSpriteComponent.SetSprite` _rendercomponent _sprite)
  (`SceneComponent.SetMobility` _rendercomponent "Movable"))

(fn `UpdatePositions`
  (locals (CameraVelocityX :type "Float (double-precision)") (MaxLayers :type Integer :default 3))
  (bind _returnvalue_x (`KismetMathLibrary.BreakVector` (`self.K2_GetActorLocation` (`self.Fokus`))))
  (set `local.CameraVelocityX` (- _returnvalue_x (`self.LastPositionX`)))
  (set `self.LastPositionX` _returnvalue_x)
  (for _array_element (`self.ParallaxObjects`)
    (`SceneComponent.K2_AddRelativeLocation` (`PaperSpriteActor.RenderComponent` _array_element) (`KismetMathLibrary.MakeVector` (* (`local.CameraVelocityX`) (* (`/Game/Blueprints/Level/BP_ParallaxObject.Layer` _array_element) (`self.LayerMultiplier`)))) false false)))

(fn `UserConstructionScript`)