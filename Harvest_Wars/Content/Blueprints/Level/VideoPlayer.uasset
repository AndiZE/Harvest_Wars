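; VideoPlayer plays the Harvest Wars intro video, then loads the Level01-Persistent level.
; On BeginPlay it adds the WBP_IntroVideo widget to the viewport and, after a short delay, opens the media source on its player.
; The level opens when playback reaches the end, or when Tick detects Space or the gamepad bottom face button while the widget's CanSkip flag is set.
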(event `self.ReceiveBeginPlay`
  (bind _returnvalue (`|CreateWidget` "/Game/Movies/WBP_IntroVideo.WBP_IntroVideo_C"))
  (bind _output_get (set `self.VideoWidget` _returnvalue))
  (`UserWidget.AddToViewport` _output_get 0)
  (`KismetSystemLibrary.Delay` 0.5)
  (`MediaPlayer.OpenSource` (`self.Player`) "/Game/Movies/HarvestWarsIntroVideo.HarvestWarsIntroVideo"))

(event `self.ReceiveTick`
  (params (DeltaSeconds :type "Float (single-precision)"))
  (bind _returnvalue (`GameplayStatics.GetPlayerController` 0))
  (if (and (or (`PlayerController.WasInputKeyJustPressed` _returnvalue "Gamepad_FaceButton_Bottom") (`PlayerController.WasInputKeyJustPressed` _returnvalue "SpaceBar")) (`/Game/Movies/WBP_IntroVideo.CanSkip` (`self.VideoWidget`)))
    (`GameplayStatics.OpenLevel` "Level01-Persistent" :!label _label)))

(event `self.Player.OnEndReached`
  (goto _label))

(fn `UserConstructionScript`)