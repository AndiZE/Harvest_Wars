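; Level trigger that spawns a wave of carrot and garlic enemies once the player count inside it matches the game instance's MaxPlayers.
; It fires once, locking the level camera on its focus point and starting a looping timer per enemy type.
; Carrots spawn randomly within the box, garlics at left/right points via a FlipFlop, and each registers with BP_AIHandler.
; When both counts run out, it allows camera unlock through BP_LevelSetup.
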(event `self.ReceiveBeginPlay`
  ;[1 1 1] Init
  (bind _outactors (`GameplayStatics.GetAllActorsOfClass` "/Game/Blueprints/AI/BP_AIHandler.BP_AIHandler_C"))
  (set `self.AIHandler` (`|GetArrayItem` _outactors)))

(event `self.CollisionComponent.OnComponentBeginOverlap`
  (params (OverlappedComponent :type "PrimitiveComponent Object Reference") (OtherActor :type "Actor Object Reference") (OtherComp :type "PrimitiveComponent Object Reference") (OtherBodyIndex :type Integer) (bFromSweep :type Boolean) (SweepResult :type "HitResult Structure (by ref)"))
  ;[1 1 1] Area Enter
  (bind _asbp_base_player_character (cast `/Game/Blueprints/Character/BP_BasePlayerCharacter` OtherActor))
  (if (`self.SpawnAviable`)
    (`KismetArrayLibrary.Array_AddUnique` (`self.Players`) _asbp_base_player_character)
    (`self.CheckForReady`)))

(event `self.CollisionComponent.OnComponentEndOverlap`
  (params (OverlappedComponent :type "PrimitiveComponent Object Reference") (OtherActor :type "Actor Object Reference") (OtherComp :type "PrimitiveComponent Object Reference") (OtherBodyIndex :type Integer))
  ;[1 1 1] Area Exit
  (bind _asbp_base_player_character (cast `/Game/Blueprints/Character/BP_BasePlayerCharacter` OtherActor))
  (if (`self.SpawnAviable`)
    (`KismetArrayLibrary.Array_RemoveItem` (`self.Players`) _asbp_base_player_character)))

(event `CheckForReady`
  ;[1 1 1] Spawn Event Start
  (bind _asbp_game_instance (cast `/Game/Gamemode/BP_GameInstance` (`GameplayStatics.GetGameInstance`)))
  (if (and (== (`/Game/Gamemode/BP_GameInstance.MaxPlayers` _asbp_game_instance) (`KismetArrayLibrary.Array_Length` (`self.Players`))) (`self.SpawnAviable`))
    (set `self.SpawnAviable` false)
    (bind _returnvalue (`KismetSystemLibrary.K2_SetTimerDelegate` (delegate `CheckSpawnGarlic`) (`self.SpawnIntervalGarlic`) true))
    (set `self.TimeHandleGarlic` _returnvalue)
    (bind _returnvalue_2 (`KismetSystemLibrary.K2_SetTimerDelegate` (delegate `CheckSpawnCarrot`) (`self.SpawnIntervalCarrot`) true))
    (set `self.TimeHandleCarrot` _returnvalue_2)
    ;[1 1 1] LockCamera
    (bind _outactors (`GameplayStatics.GetAllActorsOfClass` "/Game/Blueprints/Level/BP_LevelSetup.BP_LevelSetup_C"))
    (`/Game/Blueprints/Level/BP_LevelSetup.LockCamera` (`|GetArrayItem` _outactors) (`SceneComponent.K2_GetComponentLocation` (`self.CameraFocusPoint`)))))

(event `CheckSpawnCarrot`
  ;[1 1 1] Spawn Event Start
  (if (> (`self.NumCarrots`) 0)
    (`/Engine/EditorBlueprintResources/StandardMacros.DecrementInt` (`self.NumCarrots`)
      (:`  `
        (`self.SpawnCarrot`)))
    (else
      (`KismetSystemLibrary.K2_ClearAndInvalidateTimerHandle` (`self.TimeHandleCarrot`))
      (if (not (`KismetSystemLibrary.K2_IsValidTimerHandle` (`self.TimeHandleGarlic`)))
        (bind _outactors (`GameplayStatics.GetAllActorsOfClass` "/Game/Blueprints/Level/BP_LevelSetup.BP_LevelSetup_C" :!label _label))
        (set `/Game/Blueprints/Level/BP_LevelSetup.canUnlockCamera` true (`|GetArrayItem` _outactors))))))

(event `CheckSpawnGarlic`
  ;[1 1 1] Spawn Event Start
  (if (> (`self.NumGarlics`) 0)
    (`/Engine/EditorBlueprintResources/StandardMacros.DecrementInt` (`self.NumGarlics`)
      (:`  `
        (`self.SpawnGarlic`)))
    (else
      (`KismetSystemLibrary.K2_ClearAndInvalidateTimerHandle` (`self.TimeHandleGarlic`))
      (if (not (`KismetSystemLibrary.K2_IsValidTimerHandle` (`self.TimeHandleCarrot`)))
        (goto _label)))))

(event `SpawnCarrot`
  ;[1 1 1] Carrot
  (bind _asbox_collision (cast `BoxComponent` (`self.CollisionComponent`)))
  (bind _returnvalue (`|SpawnActorFromClass` "/Game/Blueprints/AI/BP_Carrot.BP_Carrot_C" (`KismetMathLibrary.MakeTransform` (`KismetMathLibrary.MakeVector` (.x (`KismetMathLibrary.RandomPointInBoundingBox` (`SceneComponent.K2_GetComponentLocation` _asbox_collision) (`BoxComponent.GetScaledBoxExtent` _asbox_collision))) (.y (`KismetMathLibrary.RandomPointInBoundingBox` (`SceneComponent.K2_GetComponentLocation` _asbox_collision) (`BoxComponent.GetScaledBoxExtent` _asbox_collision))) 90.0) (struct :`Roll` -90.0)) "AlwaysSpawn" "OverrideRootScale" null null))
  (`/Game/Blueprints/AI/BP_Carrot.Spawn` _returnvalue)
  (`/Game/Blueprints/AI/BP_AIHandler.EnemyAdded` (`self.AIHandler`) _returnvalue))

(event `SpawnGarlic`
  ;[1 1 1] Garlic
  (bind _isa (`/Engine/EditorBlueprintResources/StandardMacros.FlipFlop`)
    (:`A`
      _)
    (:`B`
      _))
  (bind _returnvalue (`|SpawnActorFromClass` "/Game/Blueprints/AI/BP_Garlic.BP_Garlic_C" (`KismetMathLibrary.MakeTransform` (`KismetMathLibrary.MakeVector` (.x (`SceneComponent.K2_GetComponentLocation` (select `bool` _isa :`false` (`self.SpawnLeft`) :`true` (`self.SpawnRight`)))) (.y (`SceneComponent.K2_GetComponentLocation` (select `bool` _isa :`false` (`self.SpawnLeft`) :`true` (`self.SpawnRight`)))) 90.0) (struct :`Roll` -90.0)) "AlwaysSpawn" "OverrideRootScale" null null))
  (`/Game/Blueprints/AI/BP_AIHandler.EnemyAdded` (`self.AIHandler`) _returnvalue))

(fn `UserConstructionScript`)