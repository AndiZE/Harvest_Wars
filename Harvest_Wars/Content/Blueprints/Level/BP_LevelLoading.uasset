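; BP_LevelLoading swaps streamed levels, using the current and previous level names stored in BP_GameInstance.
; ChangeLevel shifts LevelToLoad into LevelToUnload and records the new name, returning whether the game instance cast succeeded; it does not trigger streaming itself.
; StreamNewLevel loads the target as visible with blocking, then unloads the previous level without blocking if one is set, calling load-finished and unload-finished notifications after each step.
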(event `StreamNewLevel`
  (bind _asbp_game_instance (cast `/Game/Gamemode/BP_GameInstance` (`GameplayStatics.GetGameInstance`)))
  (`GameplayStatics.LoadStreamLevel` (`/Game/Gamemode/BP_GameInstance.LevelToLoad` _asbp_game_instance) true true)
  (`self.OnStreamLoadFinished`)
  (bind _leveltounload (`/Game/Gamemode/BP_GameInstance.LevelToUnload` _asbp_game_instance))
  (if (!= _leveltounload "None")
    (`GameplayStatics.UnloadStreamLevel` _leveltounload)
    (`self.OnStreamUnloadFinished`)))

(fn `ChangeLevel`
  (params (LevelName :type Name))
  (returns (Success :type Boolean))
  (bind _asbp_game_instance (cast `/Game/Gamemode/BP_GameInstance` (`GameplayStatics.GetGameInstance`))
    (:`then`
      (set `/Game/Gamemode/BP_GameInstance.LevelToUnload` (`/Game/Gamemode/BP_GameInstance.LevelToLoad` _asbp_game_instance) _asbp_game_instance)
      (set `/Game/Gamemode/BP_GameInstance.LevelToLoad` LevelName _asbp_game_instance)
      (return true))
    (:`CastFailed`
      (return false))))

(fn `UserConstructionScript`)