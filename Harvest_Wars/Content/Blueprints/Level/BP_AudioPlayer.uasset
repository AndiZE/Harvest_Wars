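; BP_AudioPlayer is a level actor that plays the full soundtrack on BeginPlay and applies the player's saved volume settings.
; It loads the AudioConfig save slot, or creates and saves a default one if none exists, then reads master, music and SFX volumes.
; SetVolumes pushes them as sound class overrides on a sound mix, multiplying music and SFX by master rather than propagating to child classes.
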(event `self.ReceiveBeginPlay`
  (bind _player (`self.Player`))
  (`self.Load Audio Config`)
  (set `AudioComponent.Sound` "/Game/Assets/UI/Sound/HW_Soundtrack_Full_Version.HW_Soundtrack_Full_Version" _player)
  (`AudioComponent.Play` _player 0.0))

(event `Load Audio Config`
  ;[1 1 1] Load Audio Config
  (bind _returnvalue (`GameplayStatics.LoadGameFromSlot` "AudioConfig"))
  (`/Engine/EditorBlueprintResources/StandardMacros.IsValid` _returnvalue
    (:`Is Valid`
      (bind _asaudio_config (cast `/Game/Audio/AudioConfig` _returnvalue))
      (bind (_master _music _sfx) (`/Game/Audio/AudioConfig.LoadAudio` _asaudio_config))
      (`self.SetVolumes` _master _music _sfx))
    (:`Is Not Valid`
      (bind _returnvalue_2 (`GameplayStatics.CreateSaveGameObject` "/Game/Audio/AudioConfig.AudioConfig_C"))
      (`GameplayStatics.SaveGameToSlot` _returnvalue_2 "AudioConfig")
      (bind (_master_2 _music_2 _sfx_2) (`/Game/Audio/AudioConfig.LoadAudio` _returnvalue_2))
      (`self.SetVolumes` _master_2 _music_2 _sfx_2))))

(event `SetVolumes`
  (params (Master :type "Float (double-precision)") (Music :type "Float (double-precision)") (SFX :type "Float (double-precision)"))
  ;[1 1 1] Apply Volume
  (`|ExecutionSequence`
    (:`then_0`
      (`GameplayStatics.SetSoundMixClassOverride` "/Game/Audio/SoundMix.SoundMix" "/Game/Audio/SC_Master.SC_Master" Master 1.0 0.0 false))
    (:`then_1`
      (`GameplayStatics.SetSoundMixClassOverride` "/Game/Audio/SoundMix.SoundMix" "/Game/Audio/SC_Music.SC_Music" (* Master Music) 1.0 0.0 false))
    (:`then_2`
      (`GameplayStatics.SetSoundMixClassOverride` "/Game/Audio/SoundMix.SoundMix" "/Game/Audio/SC_SFX.SC_SFX" (* Master SFX) 1.0 0.0 false))))

(fn `UserConstructionScript`)