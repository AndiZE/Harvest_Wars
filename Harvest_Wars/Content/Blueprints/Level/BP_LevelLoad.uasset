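; Level transition trigger that opens the level named by LevelName once all players stand inside its collision volume.
; Overlap events add and remove player characters in Players, and LoadLevel fires when that count equals MaxPlayers from BP_GameInstance.
; LoadLevel optionally saves each player character's data, then plays a WBP_LoadingFade fade.
; The fade's finished event opens the new level.
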(event `LoadLevel`
  (if (`self.SavePlayerData`)
    (bind _outactors (`GameplayStatics.GetAllActorsOfClass` "/Game/Blueprints/Character/BP_BasePlayerCharacter.BP_BasePlayerCharacter_C"))
    (for _array_element _outactors
      (`/Game/Blueprints/Character/BP_BasePlayerCharacter.SavePlayerData` _array_element)))
  (bind _returnvalue (`|CreateWidget` "/Game/UI/InGame/WBP_LoadingFade.WBP_LoadingFade_C"))
  (`UserWidget.AddToViewport` _returnvalue 0)
  (`/Game/UI/InGame/WBP_LoadingFade.LevelEnd` _returnvalue 0.5)
  (add `/Game/UI/InGame/WBP_LoadingFade.OnFadeFinished` _returnvalue (delegate `FadeFinished`)))

(event `FadeFinished`
  (`GameplayStatics.OpenLevel` (`self.LevelName`)))

(event `self.CollisionComponent.OnComponentBeginOverlap`
  (params (OverlappedComponent :type "PrimitiveComponent Object Reference") (OtherActor :type "Actor Object Reference") (OtherComp :type "PrimitiveComponent Object Reference") (OtherBodyIndex :type Integer) (bFromSweep :type Boolean) (SweepResult :type "HitResult Structure (by ref)"))
  (bind _players (`self.Players`))
  ;[1 1 1] Area Enter
  (bind _asbp_base_player_character (cast `/Game/Blueprints/Character/BP_BasePlayerCharacter` OtherActor))
  (`KismetArrayLibrary.Array_AddUnique` _players _asbp_base_player_character)
  (bind _asbp_game_instance (cast `/Game/Gamemode/BP_GameInstance` (`GameplayStatics.GetGameInstance`)))
  (if (== (`/Game/Gamemode/BP_GameInstance.MaxPlayers` _asbp_game_instance) (`KismetArrayLibrary.Array_Length` _players))
    (`self.LoadLevel`)))

(event `self.CollisionComponent.OnComponentEndOverlap`
  (params (OverlappedComponent :type "PrimitiveComponent Object Reference") (OtherActor :type "Actor Object Reference") (OtherComp :type "PrimitiveComponent Object Reference") (OtherBodyIndex :type Integer))
  ;[1 1 1] Area Exit
  (bind _asbp_base_player_character (cast `/Game/Blueprints/Character/BP_BasePlayerCharacter` OtherActor))
  (`KismetArrayLibrary.Array_RemoveItem` (`self.Players`) _asbp_base_player_character))

(fn `UserConstructionScript`)