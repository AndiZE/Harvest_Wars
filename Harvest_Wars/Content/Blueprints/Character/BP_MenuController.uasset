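; BP_MenuController is a player controller for menus that turns gameplay input actions into menu button events.
; On BeginPlay it sets Game and UI input mode.
; Attack, SpecialAttack and Menu presses fire the Confirm, Cancel and Start dispatchers, each passing the player's controller ID.
; Init caches that ID from a controller passed in, as a comment notes a self reference is buggy.
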(event `self.ReceiveBeginPlay`
  (`WidgetBlueprintLibrary.SetInputMode_GameAndUIEx` self null "DoNotLock" false))

(event `InputAction|Attack` :consume false
  (params (Key :type "Key Structure"))
  (:`Pressed`
    (`self.OnButtonConfirm` (`self.PlayerControllerID`))))

(event `InputAction|SpecialAttack` :consume false
  (params (Key :type "Key Structure"))
  (:`Pressed`
    (`self.OnButtonCancel` (`self.PlayerControllerID`))))

(event `InputAction|Menu` :consume false
  (params (Key :type "Key Structure"))
  (:`Pressed`
    (`self.OnButtonStart` (`self.PlayerControllerID`))))

(fn `Init`
  (params (Controller :type "PlayerController Object Reference"))
  (set `self.PlayerControllerID` (`GameplayStatics.GetPlayerControllerID` Controller)))

(fn `UserConstructionScript`)