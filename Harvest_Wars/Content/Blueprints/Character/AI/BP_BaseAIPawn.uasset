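; Base Paper2D enemy pawn that faces and attacks the player, using Armor for flipbooks and speed.
; A spawned helper sprite actor, attached to the player by AttackPlayer, serves as the Blackboard attack position.
; Attacks use either a weapon timeline with weapon-supplied curves or a body flipbook with a trigger frame, dealing DamageComponent damage once per swing.
; Death spawns data-table loot, notifies the AI handler and destroys the pawn.
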(event `self.ReceiveBeginPlay`
  (bind (_weapon_name _weapon_category _weapon_mindamage _weapon_maxdamage _weapon_attackspeed _weapon_range _weapon_icon _weapon_sprite _weapon_animationcurvesnormal) (break `/Game/Blueprints/Item/Weapon/Weapon` (`self.Weapon`)))
  (`parent.ReceiveBeginPlay`)
  (`|ExecutionSequence`
    (:`then_0`
      ;[1 1 1] Spawns Targeting Helper Actor
      (bind _returnvalue (`|SpawnActorFromClass` "/Script/Paper2D.PaperSpriteActor" (`KismetMathLibrary.MakeTransform` (0.0 0.0 0.0) (struct :`Roll` -90.0)) "AlwaysSpawn" "OverrideRootScale" null null))
      (`self.SetActorEnableCollision` _returnvalue false)
      (bind _rendercomponent (`PaperSpriteActor.RenderComponent` _returnvalue))
      (`SceneComponent.SetMobility` _rendercomponent "Movable")
      (`PaperSpriteComponent.SetSprite` _rendercomponent null) ; Debug Purpose
      (bind _output_get (set `self.TargetPosition` _returnvalue))
      (`BlackboardComponent.SetValueAsObject` (`AIBlueprintHelperLibrary.GetBlackboard` null) (`self.BBKey_AttackPosition`) _output_get)
      ;[1 1 1] HealthUpdate
      (add `/Game/Blueprints/Character/HealthComponent.OnHealthChanged` (`self.HealthComponent`) (delegate `OnHealthChanged`)))
    (:`then_1`
      ;[1 1 1] On Death Binding
      (add `/Game/Blueprints/Character/HealthComponent.OnDie` (`self.HealthComponent`) (`|CreateDelegate` :!event `OnDie`))
      (`self.InitTimeline` _weapon_animationcurvesnormal _weapon_attackspeed)
      (`/Game/Blueprints/Character/DamageComponent.Init` (`self.DamageComponent`) (`self.Weapon`))
      (`/Game/Blueprints/Character/HealthComponent.LoadFromInstance` (`self.HealthComponent`) 0 (`self.Armor`))
      (bind _outactors (`GameplayStatics.GetAllActorsOfClass` "/Game/Blueprints/Character/AI/BP_AIHandler.BP_AIHandler_C")))))

(event `OnHealthChanged`
  (params (CurrentHealth :type Integer) (MaxHealth :type Integer))
  ;[1 1 1] HealthUpdate
)

(event `AttackFrameUpdate`
  (bind _sprite (`self.Sprite`))
  ;[1 1 1] FlipbookAttack
  (if (`self.FlipBookIsAttacking`)
    (if (>= (`PaperFlipbookComponent.GetPlaybackPositionInFrames` _sprite) (- (`PaperFlipbookComponent.GetFlipbookLengthInFrames` _sprite) 1))
      (`self.ResetAttack`)
      (goto _label :!via `Reset`)
      (elif (>= (`PaperFlipbookComponent.GetPlaybackPositionInFrames` (`self.Sprite`)) (`self.AttackTriggerFrame`))
        (`/Engine/EditorBlueprintResources/StandardMacros.DoOnce` false :!label _label
          (:`Completed`
            (`self.AttackEnemy`)))))))

(event `AttackAnimation`
  (bind _sprite (`self.Sprite`))
  ;[1 1 1] Attack Animation Weapon
  (if (`self.HasWeapon`)
    (bind (_direction _rotation _location) (`Timeline|AttackTimeline` :!via `PlayFromStart`)
      (:`Update`
        (`SceneComponent.K2_SetRelativeLocationAndRotation` (`self.WeaponSprite`) _location (`KismetMathLibrary.MakeRotator` 0.0 _rotation) false false))
      (:`Finished`
        (`self.ResetAttack`)
        (goto _label_2 :!via `Reset`))
      (:`AttackTrigger`
        (`/Engine/EditorBlueprintResources/StandardMacros.DoOnce` false :!label _label_2
          (:`Completed`
            (`self.AttackEnemy`)))))
    (else
      (`PaperFlipbookComponent.SetFlipbook` _sprite (`self.AttackAnimFlipbook`))
      (`PaperFlipbookComponent.SetLooping` _sprite false)
      (set `self.FlipBookIsAttacking` true))))

(event `self.ReceiveTick`
  (params (DeltaSeconds :type "Float (single-precision)"))
  (bind ((`MovementBonus_21_5708F7C0431C71F2FEE017A94FD6D62D` _movementbonus)) (break `/Game/Blueprints/Item/Armor/Armor` (`self.Armor`)))
  (bind _returnvalue_x (`KismetMathLibrary.BreakVector` (`self.K2_GetActorLocation` (`self.TargetPlayer`))))
  (bind _returnvalue_x_2 (`KismetMathLibrary.BreakVector` (`self.K2_GetActorLocation` self)))
  (bind _returnvalue (`BlackboardComponent.GetValueAsBool` (`AIBlueprintHelperLibrary.GetBlackboard` null) (`self.BBKey_IsAttacking`)))
  (bind _velocity_x (`KismetMathLibrary.BreakVector` (`MovementComponent.Velocity` (`self.CharacterMovement`))))
  (bind _velocity_x_2 (`KismetMathLibrary.BreakVector` (`MovementComponent.Velocity` (`self.CharacterMovement`))))
  ;[1 1 1] Set Moving Direction Bool
  (if (`BlackboardComponent.GetValueAsBool` (`AIBlueprintHelperLibrary.GetBlackboard` self) (`self.BBKey_SpawnFinished`))
    (if (not (`self.FlipBookIsAttacking`))
      (`self.UpdateAnimation`))
    (set `CharacterMovementComponent.MaxWalkSpeed` (select `bool` _returnvalue :`false` _movementbonus :`true` (* _movementbonus 1.7)) (`self.CharacterMovement`))
    (if _returnvalue
      ;[1 1 1] Facing to Player, ingore Velocity Movement
      (bind _output_get (set `self.IsRight` (< (- _returnvalue_x_2 _returnvalue_x) 0.0)))
      (if _output_get
        (`self.K2_SetActorRotation` (struct :`Pitch` 180.0 :`Roll` -90.0))
        (else
          (`self.K2_SetActorRotation` (struct :`Roll` -90.0))))
      (if (not (`self.HasWeapon`))
        (`self.AttackFrameUpdate`))
      (else
        (if (> _velocity_x_2 0.0)
          (set `self.IsRight` true)
          (elif (< _velocity_x_2 0.0)
            (set `self.IsRight` false)))
        ;[1 1 1] Set Charater Moving Rotation
        (`/Engine/EditorBlueprintResources/StandardMacros.CompareFloat` _velocity_x
          (:`>`
            (`self.K2_SetActorRotation` (struct :`Pitch` 180.0 :`Roll` -90.0) :!label _label_3))
          (:`==`
            (if (`self.IsRight`)
              (goto _label_3)
              (else
                (`self.K2_SetActorRotation` (struct :`Roll` -90.0) :!label _label_4))))
          (:`<`
            (goto _label_4)))))))

(event `self.PawnSensing.OnSeePawn`
  (params (Pawn :type "Pawn Object Reference"))
  ;[1 1 1] Player Contact
)

(event `AttackPlayer`
  (params (player :type "/Game/Blueprints/Character/BP_BasePlayerCharacter Object Reference"))
  (bind _returnvalue (`AIBlueprintHelperLibrary.GetBlackboard` null))
  ;[1 1 1] Player Contact
  (if (and (`/Game/Blueprints/Character/HealthComponent.IsAlive` (`/Game/Blueprints/Character/BP_BasePawn.HealthComponent` player)) (not (`KismetSystemLibrary.IsValid` (`self.TargetPlayer`))))
    (bind _output_get (set `self.TargetPlayer` player))
    (`BlackboardComponent.SetValueAsObject` _returnvalue (`self.BBKey_Player`) _output_get)
    (`self.K2_AttachToActor` (`self.TargetPosition`) player "None" "KeepRelative" "SnapToTarget" "SnapToTarget" true)
    (`BlackboardComponent.SetValueAsBool` _returnvalue (`self.BBKey_FoundPlayer`) true)))

(event `UpdateAnimation`
  (bind _sprite (`self.Sprite`))
  (bind ((`AnimationIdle_43_B724D8634A0D0C04C3E03CBF3D4E39EC` _animationidle) (`AnimationWalk_46_C000BCE843F95D79EF951392215D401D` _animationwalk)) (break `/Game/Blueprints/Item/Armor/Armor` (`self.Armor`)))
  ;[1 1 1] Movement & Die Animations
  (if (`/Game/Blueprints/Character/HealthComponent.IsAlive` (`self.HealthComponent`))
    (`PaperFlipbookComponent.SetFlipbook` (`self.Sprite`) (select `bool` (> (`KismetMathLibrary.VSize` (`self.GetVelocity`)) 0.0) :`false` _animationidle :`true` _animationwalk))
    (else
      (`PaperFlipbookComponent.SetLooping` _sprite false)
      (`PaperFlipbookComponent.SetFlipbook` _sprite (`.AnimationDie_47_63D0E9764C8451B32C25E3AA126967B3` (break `/Game/Blueprints/Item/Armor/Armor` (`self.Armor`))))
      (`KismetSystemLibrary.PrintString` "Hello" true true (struct :`R` 1.0 :`B` 0.008842 :`A` 1.0)))))

(fn `AttackEnemy`
  (bind _asbp_base_player_character (cast `/Game/Blueprints/Character/BP_BasePlayerCharacter` (`BlackboardComponent.GetValueAsObject` (`AIBlueprintHelperLibrary.GetBlackboard` null) (`self.BBKey_Player`))))
  (`/Game/Blueprints/Character/HealthComponent.DamageRecieve` (`/Game/Blueprints/Character/BP_BasePawn.HealthComponent` _asbp_base_player_character) (`/Game/Blueprints/Character/DamageComponent.CalculateDamage` (`self.DamageComponent`))))

(fn `InitTimeline`
  (params (AttackCurves :type "/Game/Blueprints/Item/Weapon/AttackAnimationCurves Structure") (Attackspeed :type "Float (double-precision)"))
  (bind (_location _rotation _attacktrigger) (break `/Game/Blueprints/Item/Weapon/AttackAnimationCurves` AttackCurves))
  (`TimelineComponent.SetPlayRate` (`self.AttackTimeline`) (/ 1.0 Attackspeed))
  (`TimelineComponent.SetFloatCurve` (`self.AttackTimeline`) _rotation (`self.Timeline_Rotation`))
  (`TimelineComponent.SetFloatCurve` (`self.AttackTimeline`) _attacktrigger (`self.Timeline_AttackTrigger`))
  (`TimelineComponent.SetVectorCurve` (`self.AttackTimeline`) _location (`self.Timeline_Location`)))

(fn `MoveToNoise`
  (params (Location :type "Vector Structure"))
  (locals (IsValidLocation :type Boolean :default true) (LookingRadius :type "Float (double-precision)" :default 0.0) (ValidLocation :type "Vector Structure"))
  (bind (_randomlocation _returnvalue) (`NavigationSystemV1.K2_GetRandomReachablePointInRadius` (`local.Location`) (`local.LookingRadius`) null null))
  (if (`AIBlueprintHelperLibrary.IsValidAILocation` Location)
    (`NavigationSystemV1.FindPathToLocationSynchronously` (`self.K2_GetActorLocation`) (`local.Location`) null null)
    (else
      (while (`local.IsValidLocation`)
        (set `local.LookingRadius` (+ (`local.LookingRadius`) 10.0))
        (set `local.IsValidLocation` (not _returnvalue))
        (set `local.ValidLocation` _randomlocation))
      (`NavigationSystemV1.FindPathToLocationSynchronously` (`self.K2_GetActorLocation`) (`local.ValidLocation`) null null))))

(fn `OnDie`
  (bind (_lootpool_datatable _lootpool_rowname) (break `DataTableRowHandle` (`self.LootPool`)))
  (`|ExecutionSequence`
    (:`then_0`
      (bind _returnvalue (`|GetDataTableRow` _lootpool_datatable _lootpool_rowname)
        (:`then`
          (`/Game/Blueprints/Item/Loot/BPML_LootHelper.SpawnLoot` _returnvalue (`self.K2_GetActorLocation`) 50.0
            (:`Out`
              (`self.K2_DestroyActor` (`self.TargetPosition`))
              (`/Game/Blueprints/Character/AI/BP_AIHandler.OnEnemyDied` (`self.AiHandler`) self))))))
    (:`then_1`
      (`self.K2_DestroyActor`))))

(fn `ResetAttack`
  (if (`self.HasWeapon`)
    (`SceneComponent.K2_SetRelativeLocationAndRotation` (`self.WeaponSprite`) (0.0 0.0 0.0) (`KismetMathLibrary.MakeRotator` 0.0) false false)
    (`self.AttackFinished`)
    (else
      (`PaperFlipbookComponent.SetLooping` (`self.Sprite`) true)
      (`self.AttackFinished`)
      (set `self.FlipBookIsAttacking` false))))

(fn `UpdateTargetOffset`
  (params (isRightSide :type Boolean))
  (bind (_returnvalue_x _returnvalue_y) (`KismetMathLibrary.BreakVector` (`self.K2_GetActorLocation`)))
  (bind (_weapon_name _weapon_category _weapon_mindamage _weapon_maxdamage _weapon_attackspeed _weapon_range) (break `/Game/Blueprints/Item/Weapon/Weapon` (`self.Weapon`)))
  (bind (_returnvalue_x_2 _returnvalue_y_2) (`KismetMathLibrary.BreakVector` (`self.K2_GetActorLocation` (`self.TargetPlayer`))))
  (`self.K2_SetActorRelativeLocation` (`self.TargetPosition`) (`KismetMathLibrary.MakeVector` (`KismetMathLibrary.FClamp` (- _returnvalue_x _returnvalue_x_2) (* _weapon_range -1.0) _weapon_range) 0.0 (`KismetMathLibrary.FClamp` (- _returnvalue_y_2 _returnvalue_y) -200.0 200.0)) false false))

(fn `UserConstructionScript`)