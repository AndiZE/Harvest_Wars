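; Ranged AI pawn that attacks by firing salvos of projectiles left or right along the X axis.
; AttackEnemy starts a looping timer that spawns a BP_BaseProjectile at Weapon0 on each tick of the timer, with random damage and direction set by IsRight.
; A counter stops the timer once the salvo length is reached, then resets and calls ResetAttack.
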(event `self.AttackEnemy`
  (bind _returnvalue (`KismetSystemLibrary.K2_SetTimerDelegate` (delegate `SalveShot`) (`self.DelayShot`) true))
  (set `self.Shot_Timer` _returnvalue))

(event `SalveShot`
  (bind _returnvalue (`|SpawnActorFromClass` "/Game/Blueprints/Item/Weapon/BP_BaseProjectile.BP_BaseProjectile_C" (`KismetMathLibrary.MakeTransform` (`SceneComponent.K2_GetComponentLocation` (`self.Weapon_0`)) (`KismetMathLibrary.SelectRotator` (struct :`Roll` -90.0) (struct :`Yaw` 180.0 :`Roll` -90.0) (`self.IsRight`))) "AlwaysSpawn" "OverrideRootScale" null null))
  (`/Game/Blueprints/Item/Weapon/BP_BaseProjectile.Init` _returnvalue (`KismetMathLibrary.RandomIntegerInRange` (`self.MinDamageProjectile`) (`self.MaxDamageProjectile`)) (`KismetMathLibrary.SelectVector` (1.0 0.0 0.0) (-1.0 0.0 0.0) (`self.IsRight`)))
  (bind _result (`/Engine/EditorBlueprintResources/StandardMacros.IncrementInt` (`self.ProjectileCounter`))
    (:`  `
      (if (>= _result (`self.Salve Length`))
        (`KismetSystemLibrary.K2_ClearAndInvalidateTimerHandle` (`self.Shot_Timer`))
        (set `self.ProjectileCounter` 0)
        (`self.ResetAttack`)))))

(fn `UserConstructionScript`
  (`parent.UserConstructionScript`))