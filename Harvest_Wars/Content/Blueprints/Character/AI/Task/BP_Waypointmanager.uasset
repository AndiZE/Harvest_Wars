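; Waypoint manager Blueprint that supplies random waypoint locations, apparently for AI characters.
; On BeginPlay it gathers all actors with the waypoint tag into a list without duplicates and prints how many were found.
; GetNextWaypoint returns a random waypoint's location, re-rolling while it matches the supplied current location within a small tolerance, with no guard for fewer than two distinct waypoints.
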(event `self.ReceiveBeginPlay`
  (bind _outactors (`GameplayStatics.GetAllActorsWithTag` (`self.WayPointTag`)))
  (for _array_element _outactors
    (if (not (`KismetArrayLibrary.Array_Contains` (`self.Waypoints`) _array_element))
      (`KismetArrayLibrary.Array_Add` (`self.Waypoints`) _array_element)))
  (`KismetSystemLibrary.PrintString` (`KismetStringLibrary.Concat_StrStr` (`KismetStringLibrary.Conv_IntToString` (`KismetArrayLibrary.Array_Length` _outactors)) " Waypoints added")))

(fn `GetNextWaypoint`
  (params (CurrentWaypoint :type "Vector Structure"))
  (returns (NextWaypoint :type "Vector Structure"))
  (locals (Variable :type "Vector Structure"))
  (bind _waypoints (`self.Waypoints`))
  (bind _returnvalue (`self.K2_GetActorLocation` (`|GetArrayItem` _waypoints (`KismetMathLibrary.RandomIntegerInRange` 0 (`KismetArrayLibrary.Array_LastIndex` _waypoints)))))
  (bind _output_get (set `local.Variable` _returnvalue))
  (while (== _output_get CurrentWaypoint :`ErrorTolerance` 0.1)
    (set `local.Variable` _returnvalue))
  (return (`local.Variable`)))

(fn `UserConstructionScript`)