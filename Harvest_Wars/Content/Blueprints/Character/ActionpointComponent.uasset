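; Character component that manages an action point pool which refills over time and can be spent.
; A looping timer adds one point per interval and pauses once the maximum is reached.
; CanSpendPoints also performs the deduction and resumes a paused timer, but as written succeeds only when the cost is at least the current points.
; Gains and deductions call ActionsPointsChanged with the new count.
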(event `self.ReceiveBeginPlay`
  (bind _returnvalue (`KismetSystemLibrary.K2_SetTimerDelegate` (delegate `PointGained`) (`self.SecondsPerPoint`) true))
  (set `self.RefillTimer` _returnvalue))

(event `PointGained`
  (bind _result (`/Engine/EditorBlueprintResources/StandardMacros.IncrementInt` (`self.currentPoints`))
    (:`  `
      (if (>= _result (`self.maxPoints`))
        (`KismetSystemLibrary.K2_PauseTimerHandle` (`self.RefillTimer`)))
      (`self.ActionsPointsChanged` (`self.currentPoints`)))))

(fn `AviablePoints`
  (returns (Points :type Integer))
  (return (`self.currentPoints`)))

(fn `CanSpendPoints`
  (params (PointCost :type Integer))
  (returns (Success :type Boolean))
  (if (>= PointCost (`self.currentPoints`))
    (set `self.currentPoints` (- (`self.currentPoints`) PointCost))
    (if (`KismetSystemLibrary.K2_IsTimerPausedHandle` (`self.RefillTimer`))
      (`KismetSystemLibrary.K2_UnPauseTimerHandle` (`self.RefillTimer`)))
    (`self.ActionsPointsChanged` (`self.currentPoints`))
    (return true)
    (else
      (return false))))