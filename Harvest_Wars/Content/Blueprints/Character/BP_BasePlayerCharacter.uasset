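; Base flipbook-sprite player character handling movement, combat, item pickup and pause menu, with movement bounded around a shared camera.
; Attacks drive a timeline sampling weapon curves to animate the hand, then branch by category; only melee deals damage, ranged and magic are placeholders.
; A four-slot inventory feeds healing consumables into HealthComponent, which updates the health bar.
; Player data saves per controller ID through the GameInstance; loading is never called here.
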(event `Movement Constrains`
  (bind (_returnvalue_x _returnvalue_y) (`KismetMathLibrary.BreakVector2D` (`WidgetLayoutLibrary.GetViewportSize`)))
  (bind _returnvalue (/ _returnvalue_x _returnvalue_y))
  (bind _returnvalue_2 (* (`self.MaxCameraWidth`) 0.4))
  ;[1 1 1] Movement Radius Constrains
  (bind _output_get (set `self.MovementRangeHorizontal` (`KismetMathLibrary.MakeVector2D` (* _returnvalue_2 -1.0) _returnvalue_2)))
  (set `self.MovementRangeVertical` (`KismetMathLibrary.MakeVector2D` (/ (`KismetMathLibrary.BreakVector2D` _output_get) _returnvalue) (/ (`.Y` (`KismetMathLibrary.BreakVector2D` _output_get)) _returnvalue))))

(event `InputAction|Item1`
  (params (Key :type "Key Structure"))
  ;[1 1 1] Item Use
  (:`Pressed`
    (`self.ActivateItem` 0)))

(event `OnDie`
  ;[1 1 1] Bind On Die
)

(event `InputAction|Item2`
  (params (Key :type "Key Structure"))
  ;[1 1 1] Item Use
  (:`Pressed`
    (`self.ActivateItem` 1)))

(event `OnHealthChanged`
  (params (CurrentHealth :type Integer) (MaxHealth :type Integer))
  ;[1 1 1] Health Changed
  (bind _aswbp_health_bar (cast `/Game/UI/WBP_HealthBar` (`WidgetComponent.GetUserWidgetObject` (`self.Healthbar`))))
  (`/Game/UI/WBP_HealthBar.UpdateHealth` _aswbp_health_bar (`KismetMathLibrary.FClamp` (/ (`KismetMathLibrary.Conv_IntToDouble` CurrentHealth) (`KismetMathLibrary.Conv_IntToDouble` MaxHealth)))))

(event `InputAction|Item3`
  (params (Key :type "Key Structure"))
  ;[1 1 1] Item Use
  (:`Pressed`
    (`self.ActivateItem` 2)))

(event `InputAction|Item4`
  (params (Key :type "Key Structure"))
  ;[1 1 1] Item Use
  (:`Pressed`
    (`self.ActivateItem` 3)))

(event `self.ReceiveBeginPlay`
  (`parent.ReceiveBeginPlay`)
  (`|ExecutionSequence`
    (:`then_0`
      ;[1 1 1] Health Changed
      (add `/Game/Blueprints/Character/HealthComponent.OnHealthChanged` (`self.HealthComponent`) (delegate `OnHealthChanged`))
      ;[1 1 1] Bind On Die
      (add `/Game/Blueprints/Character/HealthComponent.OnDie` (`self.HealthComponent`) (delegate `OnDie`))
      (`self.Movement Constrains`))
    (:`then_1`
      (`self.InitInventory`)
      (`/Game/Blueprints/Character/HealthComponent.LoadFromInstance` (`self.HealthComponent`) 0 (`self.Armor`)))))

(event `UpdateAnimation`
  ;[1 1 1] Handle Movement Animation
  (`PaperFlipbookComponent.SetFlipbook` (`self.Sprite`) (select `bool` (> (`KismetMathLibrary.VSize` (`self.GetVelocity`)) 0.0) :`false` "/Game/Assets/Character/Animation/Debug/Idle.Idle" :`true` "/Game/Assets/Character/Animation/Debug/Idle.Idle" :!type "PaperFlipbook Object Reference")))

(event `PlayAttackAnimation`
  ;[1 1 1] Play Attack Animation
  (if (not (`TimelineComponent.IsPlaying` (`self.AttackAnimation`)))
    (`Timeline|AttackAnimation` :!via `PlayFromStart`
      (:`Update`
        (`self.UpdateAttackAnimation` false))
      (:`Finished`
        (`self.UpdateAttackAnimation` true)
        (`self.Attack`)))))

(event `InputAxis|MoveRight`
  (params (AxisValue :type "Float (single-precision)"))
  (bind (_movementrangehorizontal_x _movementrangehorizontal_y) (`KismetMathLibrary.BreakVector2D` (`self.MovementRangeHorizontal`)))
  (bind (_returnvalue_x _returnvalue_y) (`KismetMathLibrary.BreakVector` (`SceneComponent.K2_GetComponentLocation` (`self.PlayerCamShared`))))
  (bind (_returnvalue_x_2 _returnvalue_y_2) (`KismetMathLibrary.BreakVector` (`SceneComponent.K2_GetComponentLocation` (`self.CapsuleComponent`))))
  (bind _returnvalue (- _returnvalue_x _returnvalue_x_2))
  ;[1 1 1] Handle movement
  (if (> AxisValue 0.0)
    (set `self.bisMovingRight` true)
    (if (> _returnvalue _movementrangehorizontal_x) :!label _label
      (`self.AddMovementInput` (1.0 0.0 0.0) AxisValue :!label _label_2))
    (elif (< AxisValue 0.0)
      (set `self.bisMovingRight` false)
      (if (< _returnvalue _movementrangehorizontal_y)
        (goto _label_2))
      (else
        (goto _label)))))

(event `self.ReceiveTick`
  (params (DeltaSeconds :type "Float (single-precision)"))
  (bind _sprite (`self.Sprite`))
  ;[1 1 1] Tick - Updates animation
  (`self.UpdateAnimation`)
  (`/Engine/EditorBlueprintResources/StandardMacros.CompareFloat` (.x (`MovementComponent.Velocity` (`self.GetMovementComponent`)))
    (:`>`
      (`SceneComponent.K2_SetRelativeRotation` :`self` _sprite :!label _label_3))
    (:`==`
      (if (`self.bisMovingRight`)
        (goto _label_3)
        (else
          (`SceneComponent.K2_SetRelativeRotation` _sprite (struct :`Yaw` 180.0) false false :!label _label_4))))
    (:`<`
      (goto _label_4))))

(event `InputAxis|MoveUp`
  (params (AxisValue :type "Float (single-precision)"))
  (bind (_movementrangevertical_x _movementrangevertical_y) (`KismetMathLibrary.BreakVector2D` (`self.MovementRangeVertical`)))
  (bind (_returnvalue_x _returnvalue_y) (`KismetMathLibrary.BreakVector` (`SceneComponent.K2_GetComponentLocation` (`self.PlayerCamShared`))))
  (bind (_returnvalue_x_2 _returnvalue_y_2) (`KismetMathLibrary.BreakVector` (`SceneComponent.K2_GetComponentLocation` (`self.CapsuleComponent`))))
  (bind _returnvalue (- _returnvalue_y _returnvalue_y_2))
  ;[1 1 1] Handle movement
  (if (> AxisValue 0.0)
    (if (< _returnvalue _movementrangevertical_y)
      (`self.AddMovementInput` (0.0 -1.0 0.0) AxisValue :!label _label_5))
    (elif (> _returnvalue _movementrangevertical_x)
      (goto _label_5))))

(event `InputAction|Interaction`
  (params (Key :type "Key Structure"))
  ;[1 1 1] Interaction
  (:`Pressed`
    (bind (_outactors _returnvalue) (`KismetSystemLibrary.SphereOverlapActors` (`self.K2_GetActorLocation` self) 50.0 (`|MakeArray` "ObjectTypeQuery2" :!type "EObjectTypeQuery Enum") "/Game/Blueprints/Item/BP_BaseItem.BP_BaseItem_C"))
    (if _returnvalue
      (message `/Game/Blueprints/Item/Interact.Interact` (`|GetArrayItem` _outactors) self))))

(event `InputAction|SpecialAttack`
  (params (Key :type "Key Structure"))
  ;[1 1 1] Special Attack
  (:`Pressed`
    (bind _success (`/Game/Blueprints/Character/ActionpointComponent.CanSpendPoints` (`self.ActionpointComponent`) 1))
    (if _success
      (`self.PlayAttackAnimation`)
      (else
        (`KismetSystemLibrary.PrintString` "Not Enough Special Point")))))

(event `InputAction|Menu`
  (params (Key :type "Key Structure"))
  (bind _returnvalue (`GameplayStatics.GetPlayerController` (`self.PlayerControllerID`)))
  ;[1 1 1] Pause Menu
  (:`Pressed`
    (bind _returnvalue_2 (`|CreateWidget` "/Game/UserInterface/MainMenu/MainMenu.MainMenu_C" _returnvalue))
    (`UserWidget.AddToViewport` _returnvalue_2 0)
    (`WidgetBlueprintLibrary.SetInputMode_UIOnlyEx` _returnvalue null)
    (set `PlayerController.bShowMouseCursor` true _returnvalue)
    (`GameplayStatics.SetGamePaused` true)))

(event `InputAction|Attack`
  (params (Key :type "Key Structure"))
  ;[1 1 1] Normal Attack
  (:`Pressed`
    (`self.PlayAttackAnimation`)))

(fn `ActivateItem`
  (params (Slot :type Integer))
  (bind _hasitem (`self.HasItemInSlot` Slot))
  (if _hasitem
    (`self.ConsumeItem` (`local.Slot`))
    (`self.ClearItemInSlot` (`local.Slot`))
    (else
      (`KismetSystemLibrary.PrintString` (`KismetStringLibrary.Concat_StrStr` "no Item in Slot " (`KismetStringLibrary.Conv_IntToString` Slot))))))

(fn `AddItemInventory`
  (params (Item :type "/Game/Blueprints/Item/Consumable/Consumable Structure"))
  (bind _item (`local.Item`))
  (for (_array_element _array_index) (`self.Inventory`)
    (if (not (> (`.Health_16_E448EF084513321BF8980B87F7804D98` (break `/Game/Blueprints/Item/Consumable/Consumable` _array_element)) 0))
      (`KismetArrayLibrary.Array_Set` (`self.Inventory`) _array_index _item)
      (`self.ItemChanged` _array_index (`.Icon_5_462E0ECC4E3489F4035CDDB1F992AF19` (break `/Game/Blueprints/Item/Consumable/Consumable` _item)))
      (break))))

(fn `Attack`
  (bind (_weapon_name _weapon_category) (break `/Game/Blueprints/Item/Weapon/Weapon` (`self.Weapon`)))
  (switch `/Game/Blueprints/Item/Weapon/WeaponCategory` _weapon_category
    (:`NewEnumerator0`
      (`self.MeeleAttack`))
    (:`NewEnumerator1`
      (`KismetSystemLibrary.PrintString` "Spawn Archer Projectile"))
    (:`NewEnumerator2`
      (`KismetSystemLibrary.PrintString` "Spawn Mage Projectile"))))

(fn `ClearItemInSlot`
  (params (Slot :type Integer))
  (bind _slot (`local.Slot`))
  (bind _structout (setmembers `/Game/Blueprints/Item/Consumable/Consumable` :`StructRef` (`|GetArrayItem` (`self.Inventory`) Slot) :`Name` "None" :`Icon` null :`Health` 0 :`IntervalDuration` 0.0 :`IntervalTick` 0))
  (`KismetArrayLibrary.Array_Set` (`self.Inventory`) _slot _structout)
  (`self.ItemChanged` _slot (`.Icon_5_462E0ECC4E3489F4035CDDB1F992AF19` (break `/Game/Blueprints/Item/Consumable/Consumable` _structout))))

(fn `ConsumeItem`
  (params (Slot :type Integer))
  (bind _output (`|GetArrayItem` (`self.Inventory`) Slot))
  (bind (_name _icon _health _intervalduration _intervaltick) (break `/Game/Blueprints/Item/Consumable/Consumable` _output))
  (if (> (`.Health_16_E448EF084513321BF8980B87F7804D98` (break `/Game/Blueprints/Item/Consumable/Consumable` _output)) 0)
    (`/Game/Blueprints/Character/HealthComponent.HealRecievedTime` (`self.HealthComponent`) _health _intervaltick _intervalduration)
    (else
      (`/Game/Blueprints/Character/HealthComponent.HealRecievedInstant` (`self.HealthComponent`) _health))))

(fn `GetArmor`
  (returns (NewParam :type "/Game/Blueprints/Item/Armor/Armor Structure"))
  (return (`self.Armor`)))

(fn `GetWeapon`
  (returns (NewParam :type "/Game/Blueprints/Item/Weapon/Weapon Structure"))
  (return (`self.Weapon`)))

(fn `HasFreeInventorySlot`
  (returns (FreeSlot :type Boolean))
  (for _array_element (`self.Inventory`)
    (if (not (> (`.Health_16_E448EF084513321BF8980B87F7804D98` (break `/Game/Blueprints/Item/Consumable/Consumable` _array_element)) 0))
      (return true)))
  (return false))

(fn `HasItemInSlot`
  (params (Slot :type Integer))
  (returns (HasItem :type Boolean))
  (return (> (`.Health_16_E448EF084513321BF8980B87F7804D98` (break `/Game/Blueprints/Item/Consumable/Consumable` (`|GetArrayItem` (`self.Inventory`) Slot))) 0)))

(fn `InitInventory`
  (bind _inventory (`self.Inventory`))
  (`KismetArrayLibrary.Array_Clear` _inventory)
  (`KismetArrayLibrary.Array_Resize` _inventory 4))

(fn `LoadPlayerData`
  (bind _asbp_game_instance (cast `/Game/Gamemode/BP_GameInstance` (`GameplayStatics.GetGameInstance`)))
  (bind _playerdata (`/Game/Gamemode/BP_GameInstance.LoadPlayerData` _asbp_game_instance (`self.PlayerControllerID`)))
  (set `self.Weapon` (break `/Game/Gamemode/PlayerSaveData` _playerdata))
  (set `self.Armor` (`.Armor_9_B498E1644ECB5A5AFA12F28BBDE989B2` (break `/Game/Gamemode/PlayerSaveData` _playerdata)))
  (set `self.Inventory` (`.Items_7_2E2C324E4B183657FBFA3F9334DAE7F8` (break `/Game/Gamemode/PlayerSaveData` _playerdata)))
  (`/Game/Blueprints/Character/HealthComponent.LoadFromInstance` (`self.HealthComponent`) (`.CurrentHealth_12_2582936F492ACC94721A78B4F234A94E` (break `/Game/Gamemode/PlayerSaveData` _playerdata)) (`self.Armor`)))

(fn `MeeleAttack`
  (bind (_origin _boxextent) (`KismetSystemLibrary.GetComponentBounds` (`self.WeaponSprite`)))
  (bind (_outactors _returnvalue) (`KismetSystemLibrary.BoxOverlapActors` _origin _boxextent (`|MakeArray` "ObjectTypeQuery3" :!type "EObjectTypeQuery Enum") "/Game/Blueprints/Character/AI/BP_BaseAIPawn.BP_BaseAIPawn_C" (`|MakeArray` self :!type "Actor Object Reference")))
  (if _returnvalue
    (bind _asbp_base_aipawn (cast `/Game/Blueprints/Character/AI/BP_BaseAIPawn` (`|GetArrayItem` _outactors)))
    (`/Game/Blueprints/Character/HealthComponent.DamageRecieve` (`/Game/Blueprints/Character/BP_BasePawn.HealthComponent` _asbp_base_aipawn) (`/Game/Blueprints/Character/DamageComponent.CalculateDamage` (`self.DamageComponent`)))))

(fn `PickupItem`
  (params (Item :type "/Game/Blueprints/Item/BP_BaseItem Object Reference"))
  (switch `/Game/Blueprints/Item/ItemType` (`/Game/Blueprints/Item/BP_BaseItem.type` Item)
    (:`NewEnumerator2`
      (bind _asbp_consumable (cast `/Game/Blueprints/Item/Consumable/BP_Consumable` Item))
      (`self.AddItemInventory` (`/Game/Blueprints/Item/Consumable/BP_Consumable.Item` _asbp_consumable)))))

(fn `SavePlayerData`
  (bind _asbp_game_instance (cast `/Game/Gamemode/BP_GameInstance` (`GameplayStatics.GetGameInstance`)))
  (`/Game/Gamemode/BP_GameInstance.SavePlayerData` _asbp_game_instance (`self.PlayerControllerID`) (make `/Game/Gamemode/PlayerSaveData` (`self.Weapon`) (`self.Armor`) (`self.Inventory`) (`/Game/Blueprints/Character/HealthComponent.GetCurrentHealth` (`self.HealthComponent`)))))

(fn `UpdateAttackAnimation`
  (params (Reset :type Boolean))
  (locals (MappedPlaybackPosition :type "Float (double-precision)"))
  (bind _mappedplaybackposition (`local.MappedPlaybackPosition`))
  (bind (_weapon_name _weapon_category _weapon_mindamage _weapon_maxdamage _weapon_attackspeed _weapon_range _weapon_sprite _weapon_animationcurves) (break `/Game/Blueprints/Item/Weapon/Weapon` (`self.Weapon`)))
  (bind (_weapon_name_2 _weapon_category_2 _weapon_mindamage_2 _weapon_maxdamage_2 _weapon_attackspeed_2 _weapon_range_2 _weapon_sprite_2 _weapon_animationcurves_2) (break `/Game/Blueprints/Item/Weapon/Weapon` (`self.Weapon`)))
  (bind _attackanimation (`self.AttackAnimation`))
  (bind (_location _rotation) (break `/Game/Blueprints/Item/Weapon/PlayerAttackAnimationCurves` _weapon_animationcurves))
  (bind (_location_2 _rotation_2) (break `/Game/Blueprints/Item/Weapon/PlayerAttackAnimationCurves` _weapon_animationcurves_2))
  (if (and (`KismetSystemLibrary.IsValid` _location_2) (`KismetSystemLibrary.IsValid` _rotation_2))
    (if Reset
      (set `local.MappedPlaybackPosition` 0.0)
      (else
        (set `local.MappedPlaybackPosition` (`KismetMathLibrary.MapRangeClamped` (`TimelineComponent.GetPlaybackPosition` _attackanimation) 0.0 (`TimelineComponent.GetTimelineLength` _attackanimation) 0.0 1.0))))
    (`SceneComponent.K2_SetRelativeLocationAndRotation` (`self.Hand`) (`CurveVector.GetVectorValue` _location _mappedplaybackposition) (`KismetMathLibrary.MakeRotator` 0.0 (`CurveFloat.GetFloatValue` _rotation _mappedplaybackposition)) false false)))

(fn `UserConstructionScript`)