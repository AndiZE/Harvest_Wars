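; Health component for characters that tracks current health against a maximum and reports changes through event dispatchers.
; Health starts at maximum on BeginPlay, and healing clamps it between one and maximum.
; DamageRecieve subtracts current health from damage, zeroing health and calling Die when the result is non-positive, otherwise storing that result, so the operands appear reversed.
; Both paths broadcast OnHealthChanged, and Die broadcasts OnDie.
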(event `self.ReceiveBeginPlay`
  (set `self.currentHealth` (`self.maxHealth`)))

(fn `DamageRecieve`
  (params (Damage :type Integer))
  (bind _maxhealth (`self.maxHealth`))
  (bind _returnvalue (- Damage (`self.currentHealth`)))
  (if (<= _returnvalue 0)
    (bind _output_get (set `self.currentHealth` 0))
    (`self.OnHealthChanged` _output_get _maxhealth)
    (`self.Die`)
    (else
      (bind _output_get_2 (set `self.currentHealth` _returnvalue))
      (`self.OnHealthChanged` _output_get_2 _maxhealth))))

(fn `Die`
  (`self.OnDie`))

(fn `HealRecieved`
  (params (Health :type Integer))
  (bind _output_get (set `self.currentHealth` (`KismetMathLibrary.Clamp` (+ Health (`self.currentHealth`)) 1 (`self.maxHealth`))))
  (`self.OnHealthChanged` _output_get (`self.maxHealth`)))