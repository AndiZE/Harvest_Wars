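; Character attribute component that derives health, regeneration, movement speed, attack speed and damage from starting class, weapon and armor.
; Init loads debug DataTable rows or the set gear, and each gear change recalculates stats and notifies listeners.
; Weapon category selects physical or magical damage.
; Incoming damage rolls evasion, applies armor reduction and fires health or death events, while Tick regenerates health.
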(event `self.ReceiveTick`
  (params (DeltaSeconds :type "Float (single-precision)"))
  (`self.UpdateRegenerations`))

(fn `ChangeArmor`
  (params (Armor :type "/Game/Blueprints/Item/Armor/Armor Structure"))
  (bind _output_get (set `self.Armor` Armor))
  (`self.RecalculateStats`)
  (`self.OnArmorChanged` _output_get))

(fn `ChangeWeapon`
  (params (Weapon :type "/Game/Blueprints/Item/Weapon/Weapon Structure"))
  (bind _output_get (set `self.Weapon` Weapon))
  (`self.RecalculateStats`)
  (`self.OnWeaponChanged` _output_get))

(fn `Die`
  (`self.OnDie`))

(fn `GetArmor`
  (returns (CharacterArmor :type "/Game/Blueprints/Item/Armor/Armor Structure"))
  (return (`self.Armor`)))

(fn `GetClassType`
  (returns (ClassType :type "/Game/Blueprints/Character/ClassCategory Enum"))
  (bind (_startingclass_name _startingclass_class) (break `/Game/Blueprints/Character/CharacterBaseStats` (`self.StartingClass`)))
  (return _startingclass_class))

(fn `GetWeaponAnimationCurves`
  (returns (AnimationCurves :type "/Game/Blueprints/Item/Weapon/PlayerAttackAnimationCurves Structure"))
  (bind (_weapon_name _weapon_category _weapon_mindamage _weapon_attackspeed _weapon_specialattackregeneration _weapon_sprite _weapon_animationcurves) (break `/Game/Blueprints/Item/Weapon/Weapon` (`self.Weapon`)))
  (return _weapon_animationcurves))

(fn `GetWeaponType`
  (returns (WeaponType :type "/Game/Blueprints/Item/Weapon/WeaponCategory Enum"))
  (bind (_weapon_name _weapon_category) (break `/Game/Blueprints/Item/Weapon/Weapon` (`self.Weapon`)))
  (return _weapon_category))

(fn `Init`
  (bind (_debugweapon_datatable _debugweapon_rowname) (break `DataTableRowHandle` (`self.DebugWeapon`)))
  (bind (_debugarmor_datatable _debugarmor_rowname) (break `DataTableRowHandle` (`self.DebugArmor`)))
  (bind (_debugstartclass_datatable _debugstartclass_rowname) (break `DataTableRowHandle` (`self.DebugStartClass`)))
  (`|ExecutionSequence`
    (:`then_0`
      (if (`self.isDebug`)
        ;[1 1 1] Debug Start
        (bind _returnvalue (`|GetDataTableRow` _debugstartclass_datatable _debugstartclass_rowname)
          (:`then`
            (set `self.StartingClass` _returnvalue)
            (bind _returnvalue_2 (`|GetDataTableRow` _debugweapon_datatable _debugweapon_rowname)
              (:`then`
                (`self.ChangeWeapon` _returnvalue_2)
                (bind _returnvalue_3 (`|GetDataTableRow` _debugarmor_datatable _debugarmor_rowname)
                  (:`then`
                    (`self.ChangeArmor` _returnvalue_3)))))))
        (else
          ;[1 1 1] Regular Init
          (`self.ChangeWeapon` (`self.Weapon`))
          (`self.ChangeArmor` (`self.Armor`)))))
    (:`then_1`
      (set `self.CriticalStrengh` (`/Game/Blueprints/Character/BaseStats.BaseCritStrengh`))
      (set `self.CriticalHit` (`/Game/Blueprints/Character/BaseStats.BaseCritChance`))
      (set `self.Evasion` (`/Game/Blueprints/Character/BaseStats.BaseEvasion`)))
    (:`then_2`
      (set `self.CurrentHealth` (`KismetMathLibrary.Conv_IntToDouble` (`self.MaxHealth`)))
      (set `self.MaxSpecialAttack` (`/Game/Blueprints/Character/BaseStats.BaseSpecialAttackPoints`))
      (set `self.CurrentSpecialAttack` (`self.MaxSpecialAttack`)))))

(fn `RecalculateStats`
  (bind _specialregeneration (`/Game/Blueprints/Character/BaseStats.BaseSpecialRegeneration`))
  (bind _strengh (`self.Strengh`))
  (bind _agility (`self.Agility`))
  (bind (_weapon_name _weapon_category) (break `/Game/Blueprints/Item/Weapon/Weapon` (`self.Weapon`)))
  (bind _weapon (`self.Weapon`))
  (bind _weapon_2 (`self.Weapon`))
  (bind (_weapon_name_2 _weapon_category_2 _weapon_mindamage _weapon_attackspeed _weapon_specialattackregeneration) (break `/Game/Blueprints/Item/Weapon/Weapon` (`self.Weapon`)))
  (bind (_weapon_name_3 _weapon_category_3 _weapon_mindamage_2 _weapon_attackspeed_2) (break `/Game/Blueprints/Item/Weapon/Weapon` (`self.Weapon`)))
  (bind (_startingclass_name _startingclass_class _startingclass_strengh _startingclass_agility _startingclass_intelligence _startingclass_health) (break `/Game/Blueprints/Character/CharacterBaseStats` (`self.StartingClass`)))
  (bind (_armor_name _armor_health _armor_damagereduction _armor_movementbonus _armor_strengh _armor_agility _armor_intelligence) (break `/Game/Blueprints/Item/Armor/Armor` (`self.Armor`)))
  (bind _physicaldamagebonus (`/Game/Blueprints/Character/BaseStats.CalculatePhysicalDamage` (`self.Strengh`)))
  (bind _magicaldamage (`/Game/Blueprints/Character/BaseStats.CalculateMacigalDamage` (`self.Intelligence`)))
  (set `self.Strengh` (+ _armor_strengh _startingclass_strengh))
  (set `self.Agility` (+ _armor_agility _startingclass_agility))
  (set `self.Intelligence` (+ _armor_intelligence _startingclass_intelligence))
  (`|ExecutionSequence`
    (:`then_0`
      (set `self.MaxHealth` (+ (+ _startingclass_health _armor_health) (`/Game/Blueprints/Character/BaseStats.CalculateLife` _strengh)))
      (set `self.LifeRegenration` (`/Game/Blueprints/Character/BaseStats.CalculateHealthReg` _strengh)))
    (:`then_1`
      (set `self.MovementSpeed` (`/Game/Blueprints/Character/BaseStats.CalcuclateMovementSpeed` _agility))
      (set `self.AttackSpeed` (* _weapon_attackspeed_2 (+ (* (`/Game/Blueprints/Character/BaseStats.CalculateAttackSpeedBonus` _agility) 0.01) 1.0))))
    (:`then_3`
      (switch `/Game/Blueprints/Item/Weapon/WeaponCategory` _weapon_category
        (:`NewEnumerator0`
          (set `self.PhysicalDamage` (make `/Game/Blueprints/Item/Weapon/DamageRange` (+ (break `/Game/Blueprints/Item/Weapon/DamageRange` (`.MinDamage_18_7443742A4DB6107510C8A1A8D2CD66FA` (break `/Game/Blueprints/Item/Weapon/Weapon` _weapon_2))) _physicaldamagebonus) (+ (`.MaximalDamage_4_9A0888C44B917EDAA82B718DA9842D62` (break `/Game/Blueprints/Item/Weapon/DamageRange` (`.MinDamage_18_7443742A4DB6107510C8A1A8D2CD66FA` (break `/Game/Blueprints/Item/Weapon/Weapon` _weapon_2)))) _physicaldamagebonus)) :!label _label)
          (set `self.MagicalDamage` (make `/Game/Blueprints/Item/Weapon/DamageRange` 0)))
        (:`NewEnumerator1`
          (goto _label))
        (:`NewEnumerator2`
          (set `self.MagicalDamage` (make `/Game/Blueprints/Item/Weapon/DamageRange` (+ (break `/Game/Blueprints/Item/Weapon/DamageRange` (`.MinDamage_18_7443742A4DB6107510C8A1A8D2CD66FA` (break `/Game/Blueprints/Item/Weapon/Weapon` _weapon))) _magicaldamage) (+ (`.MaximalDamage_4_9A0888C44B917EDAA82B718DA9842D62` (break `/Game/Blueprints/Item/Weapon/DamageRange` (`.MinDamage_18_7443742A4DB6107510C8A1A8D2CD66FA` (break `/Game/Blueprints/Item/Weapon/Weapon` _weapon)))) _magicaldamage)))
          (set `self.PhysicalDamage` (make `/Game/Blueprints/Item/Weapon/DamageRange` 0))))
      (set `self.SpecialAttackRegeneration` (+ _specialregeneration (* _specialregeneration _weapon_specialattackregeneration 0.01))))))

(fn `RecieveDamage`
  (params (Damage :type Integer))
  (locals (AbsoluteDamage :type Integer))
  (bind (_armor_name _armor_health _armor_damagereduction) (break `/Game/Blueprints/Item/Armor/Armor` (`self.Armor`)))
  (bind _damage (`local.Damage`))
  ;[1 1 1] Evasion
  (if (<= (`self.Evasion`) (`KismetMathLibrary.RandomFloatInRange` 0.0 100.0))
    ;[1 1 1] Armor Reduction
    (bind _output_get (set `local.AbsoluteDamage` (- _damage (`KismetMathLibrary.Round` (* _damage (* _armor_damagereduction 0.01))))))
    (if (> _output_get 0)
      ;[1 1 1] Reduce Health
      (bind _output_get_2 (set `self.CurrentHealth` (- (`self.CurrentHealth`) (`KismetMathLibrary.Conv_IntToDouble` (`local.AbsoluteDamage`)))))
      (if (> _output_get_2 0.0)
        ;[0.2135 1 0.1232] Inform Subscribers
        (`self.OnHealthChanged` (`KismetMathLibrary.FTrunc` (`self.CurrentHealth`)) (`self.MaxHealth`))
        (else
          ;[1 0 0] Dead
          (set `self.CurrentHealth` 0.0)
          (`self.Die`)))
      (else
        (`KismetSystemLibrary.PrintString` "Attack Absorbed")))
    (else
      (`KismetSystemLibrary.PrintString` "Attack Evaded"))))

(fn `SpendSpecialAttackCost`
  (bind _output_get (set `self.CurrentSpecialAttack` (- (`self.CurrentSpecialAttack`) (`/Game/Blueprints/Character/BaseStats.BaseSpecialAttackCost`))))
  (`self.OnSpecialPointChanged` _output_get))

(fn `UpdateRegenerations`
  (bind _output_get (set `self.CurrentHealth` (+ (`self.CurrentHealth`) (* (`self.LifeRegenration`) (`GameplayStatics.GetWorldDeltaSeconds`)))))
  (if (> _output_get (`KismetMathLibrary.Conv_IntToDouble` (`self.MaxHealth`)))
    (set `self.CurrentHealth` (`KismetMathLibrary.Conv_IntToDouble` (`self.MaxHealth`)))
    (else
      (`self.OnHealthChanged` (`KismetMathLibrary.FTrunc` (`self.CurrentHealth`)) (`self.MaxHealth`)))))