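; BP_BasePawn is a base character pawn that loads its weapon and armor from data tables.
; On BeginPlay, if EditorStart is set, EditorInit resolves the WeaponTable and ArmorTable row handles into the Weapon and Armor variables.
; Each handle is first checked against its expected table, with on-screen prints confirming the item found or warning in red about a wrong table.
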(event `self.ReceiveBeginPlay`
  (if (`self.EditorStart`)
    (`self.EditorInit`)))

(fn `EditorInit`
  (bind (_weapontable_datatable _weapontable_rowname) (break `DataTableRowHandle` (`self.WeaponTable`)))
  (bind (_armortable_datatable _armortable_rowname) (break `DataTableRowHandle` (`self.ArmorTable`)))
  (`|ExecutionSequence`
    (:`then_0`
      (if (== _weapontable_datatable "/Game/Blueprints/Item/Weapon/WeaponTable.WeaponTable")
        (bind _returnvalue (`|GetDataTableRow` "/Game/Blueprints/Item/Weapon/WeaponTable.WeaponTable" _weapontable_rowname)
          (:`then`
            (bind _output_get (set `self.Weapon` _returnvalue))
            (`KismetSystemLibrary.PrintString` (`KismetStringLibrary.Concat_StrStr` "Weapon set to: " (`KismetStringLibrary.Conv_NameToString` (`.Name_2_834043AC48351CD81016819EDA2899A3` (break `/Game/Blueprints/Item/Weapon/Weapon` _output_get)))))))
        (else
          (`KismetSystemLibrary.PrintString` (`KismetStringLibrary.Concat_StrStr` (`KismetSystemLibrary.GetDisplayName` self) " Weapon Table not correct set") true true (struct :`R` 1.0 :`A` 1.0) 10.0))))
    (:`then_1`
      (if (== _armortable_datatable "/Game/Blueprints/Item/Armor/ArmorTable.ArmorTable")
        (bind _returnvalue_2 (`|GetDataTableRow` "/Game/Blueprints/Item/Armor/ArmorTable.ArmorTable" _armortable_rowname)
          (:`then`
            (bind _output_get_2 (set `self.Armor` _returnvalue_2))
            (`KismetSystemLibrary.PrintString` (`KismetStringLibrary.Concat_StrStr` "Armor set to: " (`KismetStringLibrary.Conv_NameToString` (`.Name_8_C46CDAD94EDB0E1735BB90AC2FDEDBF4` (break `/Game/Blueprints/Item/Armor/Armor` _output_get_2)))))))
        (else
          (`KismetSystemLibrary.PrintString` (`KismetStringLibrary.Concat_StrStr` (`KismetSystemLibrary.GetDisplayName` self) " Armor Table not correct set") true true (struct :`R` 1.0 :`A` 1.0) 10.0))))))

(fn `UserConstructionScript`)