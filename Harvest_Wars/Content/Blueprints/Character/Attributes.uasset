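; Character attributes Blueprint that derives combat and resource stats from Strengh, Agility and Intelligence.
; RecalculateStats feeds each primary attribute through calculation functions: Strengh drives health, regeneration and physical damage; Agility drives endurance, movement and attack speed; Intelligence drives mana and magical damage.
; Init runs that recalculation, then sets base critical strength, critical chance and evasion.
; BeginPlay and Tick are unused, and nothing in this file calls Init.
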(fn `Init`
  (`|ExecutionSequence`
    (:`then_0`
      (`self.RecalculateStats`))
    (:`then_1`
      (set `self.CriticalStrengh` (`/Game/Blueprints/Character/BaseStats.BaseCritStrengh`))
      (set `self.CriticalHit` (`/Game/Blueprints/Character/BaseStats.BaseCritChance`))
      (set `self.Evasion` (`/Game/Blueprints/Character/BaseStats.BaseEvasion`)))))

(fn `RecalculateStats`
  (bind _strengh (`self.Strengh`))
  (bind _agility (`self.Agility`))
  (bind _intelligence (`self.Intelligence`))
  (`|ExecutionSequence`
    (:`then_0`
      (set `self.Health` (`/Game/Blueprints/Character/BaseStats.CalculateLife` _strengh))
      (set `self.LifeRegenration` (`/Game/Blueprints/Character/BaseStats.CalculateHealthReg` _strengh))
      (set `self.PhysicalDamageBonus` (`/Game/Blueprints/Character/BaseStats.CalculatePhysicalDamage` _strengh)))
    (:`then_1`
      (set `self.Endurance` (`/Game/Blueprints/Character/BaseStats.CalculateEndurance` _agility))
      (set `self.EnduraceRegenration` (`/Game/Blueprints/Character/BaseStats.CalculateEnduranceRegeneration` _agility))
      (set `self.MovementSpeed` (`/Game/Blueprints/Character/BaseStats.CalcuclateMovementSpeed` _agility))
      (set `self.AttackSpeedBonus` (`/Game/Blueprints/Character/BaseStats.CalculateAttackSpeedBonus` _agility)))
    (:`then_2`
      (set `self.MagicalDamageBonus` (`/Game/Blueprints/Character/BaseStats.CalculateMacigalDamage` _intelligence))
      (set `self.Mana` (`/Game/Blueprints/Character/BaseStats.CalculateMana` _intelligence))
      (set `self.ManaRegeneration` (`/Game/Blueprints/Character/BaseStats.CalculateManaReg` _intelligence)))))